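; Player controller that owns the scoreboard UI and relays two-player scores between the game state and the player's screen.
; On BeginPlay it caches BP_RHB_GameState, then creates the scoreboard widget after a brief delay.
; Server-named events increment each player's score on the game state, whose UpdateScore message is forwarded to an owning-client event that refreshes the widget text.
; The Score event is empty, and the ID-based branch calling those increments is disconnected.
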(event Custom|Score
  (params (ID :type Integer))
  ;[0.15 0.15 0.15 0.5] Score - From Player Character
)

(event Custom|SV_Player1Score
  ;[0.15 0.15 0.15 0.5] Score To Server
  (bind _bp_gamestate (Variables|Default|GetBP_GameState)
    (:then
      (Default|IncrementP1Score _bp_gamestate))
    (:else)))

(event Custom|SV_Player2Score
  ;[0.15 0.15 0.15 0.5] Score To Server
  (bind _bp_gamestate (Variables|Default|GetBP_GameState)
    (:then
      (Default|IncrementP2Score _bp_gamestate))
    (:else)))

(event Custom|UpdateOwningClientScore
  (params (P1Score :type Integer) (P2Score :type Integer))
  ;[0.15 0.15 0.15 0.5] Updating UI Text for Owning Client
  (bind _scoreboard_wgt (Variables|Default|GetScoreboard_wgt)
    (:then
      (Default|SetPlayer1ScoreTxt _scoreboard_wgt P1Score)
      (bind _scoreboard_wgt_2 (Variables|Default|GetScoreboard_wgt)
        (:then
          (Default|SetPlayer2ScoreTxt _scoreboard_wgt_2 P2Score))
        (:else)))
    (:else)))

(event EventBeginPlay
  ;[0.15 0.15 0.15 0.5] Begin Play
  (bind _asbp_rhb_game_state (Utilities|Casting|CastToBP_RHB_GameState (Game|GetGameState)))
  (Variables|Default|SetBP_GameState _asbp_rhb_game_state)
  (Utilities|FlowControl|Delay 0.05)
  (bind _returnvalue (UserInterface|CreateWidget "/Game/_RHB_MAIN/Blueprints/UI/WGT_Scoreboard.WGT_Scoreboard_C" (Game|GetPlayerController 0)))
  (bind _output_get (Variables|Default|SetScoreboard_wgt _returnvalue))
  (Utilities|IsValid _output_get
    (:Is%20Valid
      (UserInterface|Viewport|AddtoViewport _output_get 0))))

(event EventUpdateScore
  (params (P1Score :type Integer) (P2Score :type Integer))
  ;[0.15 0.15 0.15 0.5] MSG sent from GameState
  (CallFunction|UpdateOwningClientScore P1Score P2Score))

(fn ConstructionScript)