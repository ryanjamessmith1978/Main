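; BP_RHB_GameState is the game state for a two-player ball-and-goal match, spawning the field pieces and tracking both scores.
; BallDrop spawns the ball and two numbered goals at preset locations.
; SV_BallReset switches off collision and physics to teleport the ball back to its start, notifies the goal, then restores them.
; Score increments notify player controllers found through the BPI_UpdateScore interface, passing both totals.
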(event Custom|Increment%20P1%20Score
  (bind _result (Math|Integer|IncrementInt (Variables|Default|GetPlayer1Score))
    (:%20%20
      (Variables|Default|SetPlayer1Score _result)
      (CallFunction|UpdateScoreViaInterface))))

(event Custom|UpdateScore_via_Interface
  (bind _outactors (Actor|GetAllActorswithInterface "/Game/_RHB_MAIN/Blueprints/Interfaces/BPI_UpdateScore.BPI_UpdateScore_C"))
  (for _array_element _outactors
    (bind _asbp_rhb_player_controller (Utilities|Casting|CastToBP_RHB_PlayerController _array_element))
    (Utilities|IsValid _asbp_rhb_player_controller
      (:Is%20Valid
        (Class|BPIUpdateScore|UpdateScore(Message) _asbp_rhb_player_controller (Variables|Default|GetPlayer1Score) (Variables|Default|GetPlayer2Score))))))

(event Custom|Increment%20P2%20Score
  (bind _result (Math|Integer|IncrementInt (Variables|Default|GetPlayer2Score))
    (:%20%20
      (Variables|Default|SetPlayer2Score _result)
      (CallFunction|UpdateScoreViaInterface))))

(event Custom|Ball%20Drop
  (bind _returnvalue (Game|SpawnActorfromClass "/Game/_RHB_MAIN/Blueprints/AActors/BP_Ball.BP_Ball_C" (Math|Transform|MakeTransform (Variables|Default|GetBall%20Reset%20Pos) "0, 0, 0" "1.000000,1.000000,1.000000") "Undefined" "MultiplyWithRoot" self 0))
  (Variables|Default|Setball _returnvalue)
  (bind _returnvalue_2 (Game|SpawnActorfromClass "/Game/_RHB_MAIN/Blueprints/AActors/BP_Goal.BP_Goal_C" (Math|Transform|MakeTransform (Variables|Default|Getg1Location) "0.000000,-180.000000,0.000000" "1.000000,1.000000,1.000000") "Undefined" "MultiplyWithRoot" self 0))
  (bind _output_get (Variables|Default|Setgoal1 _returnvalue_2))
  (Default|SetGoalTxtSV _output_get 1)
  (bind _returnvalue_3 (Game|SpawnActorfromClass "/Game/_RHB_MAIN/Blueprints/AActors/BP_Goal.BP_Goal_C" (Math|Transform|MakeTransform (Variables|Default|Getg2Location) "0, 0, 0" "1.000000,1.000000,1.000000") "Undefined" "MultiplyWithRoot" self 0))
  (bind _output_get_2 (Variables|Default|Setgoal2 _returnvalue_3))
  (Default|SetGoalTxtSV _output_get_2 2))

(event Custom|SV_BallReset
  (params (ball :type BP%20Ball%20Object%20Reference) (goal :type BP%20Goal%20Object%20Reference))
  (Collision|SetActorEnableCollision ball false)
  (Collision|SetCollisionEnabled (Variables|/Script/Engine.StaticMeshActor|GetStaticMeshComponent ball) "NoCollision")
  (Physics|SetSimulatePhysics (Variables|/Script/Engine.StaticMeshActor|GetStaticMeshComponent ball) false)
  (Transformation|SetActorLocationAndRotation ball (Variables|Default|GetBall%20Reset%20Pos) "0, 0, 0" false true)
  (Default|ResettingBall goal)
  (Collision|SetActorEnableCollision ball true)
  (Collision|SetCollisionEnabled (Variables|/Script/Engine.StaticMeshActor|GetStaticMeshComponent ball) "QueryAndPhysics")
  (Physics|SetSimulatePhysics (Variables|/Script/Engine.StaticMeshActor|GetStaticMeshComponent ball) true))

(fn ConstructionScript)