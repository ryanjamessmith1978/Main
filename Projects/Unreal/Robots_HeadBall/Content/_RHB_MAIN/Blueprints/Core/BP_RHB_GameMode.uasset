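; BP_RHB_GameMode is the game mode that handles player logins and starts play by spawning the ball.
; On each PostLogin it increments the player count and stores it as the player controller's UniqueID.
; Once the count is two or more, it spawns a BP_Ball at the reset position and keeps a reference to it.
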(event EventPostLogin
  (params (NewPlayer :type Player%20Controller%20Object%20Reference))
  (bind _result (Math|Integer|IncrementInt (Variables|Default|GetNumPlayers))
    (:%20%20
      (bind _output_get (Variables|Default|SetNumPlayers _result))
      (bind _asbp_rhb_player_controller (Utilities|Casting|CastToBP_RHB_PlayerController NewPlayer))
      (Variables|/Game/_RHB_MAIN/Blueprints/Core/BP_RHB_PlayerController.BP_RHB_PlayerController_C|SetUniqueID _asbp_rhb_player_controller _output_get)
      (if (>= (Variables|Default|GetNumPlayers) 2)
        (bind _returnvalue (Game|SpawnActorfromClass "/Game/_RHB_MAIN/Blueprints/AActors/BP_Ball.BP_Ball_C" (Math|Transform|MakeTransform (Variables|Default|GetBallResetPos) "0, 0, 0" "1.000000,1.000000,1.000000") "Undefined" "MultiplyWithRoot" 0 0))
        (Variables|Default|SetBP_GameBall _returnvalue)))))

(fn ConstructionScript)