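; Player character that picks up, aims and throws a BP_RHB_GameBall.
; Right mouse grabs an overlapping ball through server/multicast events, and a looping timer holds the PhysicsHandle at ThrowPoint.
; Left mouse press plays a wind-up and previews the camera-based predicted path with spline meshes; release launches the ball on a montage notify.
; Left mouse uses debug keys that bypass the throw RPCs, whose IsGrabbed-gated calls are disconnected.
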(event Custom|Hold
  (bind _throwpoint (Variables|Default|GetThrowPoint))
  ;[0.15 0.02353 0.01607 0.5] Pickup Custom Event
  ;;[0.15 0.15 0.15 0.5] Hold
  (Utilities|Time|SetTimerbyEvent (delegate Custom|Hold) 0.01 true true)
  (Class|PhysicsHandleComponent|SetTargetLocationandRotation (Variables|Default|GetPhysicsHandle) (Transformation|GetWorldLocation _throwpoint) (Transformation|GetWorldRotation _throwpoint)))

(event Custom|ReadyToThrow_SV
  ;[0.15 0.03603 0.143 0.5] Throw Ball
  ;;[0.15 0.15 0.15 0.5] Server
  (CallFunction|ReadytoThrowMC))

(event Custom|ReadyToThrow_MC
  ;[0.15 0.03603 0.143 0.5] Throw Ball
  ;;[0.15 0.15 0.15 0.5] Wind-up Animation Montage
  ;;;[0.15 0.15 0.15 0.5] Multicast
  (Animation|Montage|PlayMontage (Variables|Character|GetMesh) "/Game/_RHB_MAIN/Animations/OneHandLoop_Anim_Montage.OneHandLoop_Anim_Montage" 0.0
    (:then
      (CallFunction|DrawCurve))))

(event Custom|Throw_SV
  ;[0.15 0.03603 0.143 0.5] Throw Ball
  (CallFunction|ThrowMC))

(event Custom|Throw_MC
  ;[0.15 0.03603 0.143 0.5] Throw Ball
  ;;[0.15 0.15 0.15 0.5] Multicast
  (Variables|Default|SetbIsGrabbed false))

(event Custom|DrawCurve
  ;[0.15 0.07911 0.1459 0.5] Splines Throw Curve - Projected path
  (bind _returnvalue (Utilities|Time|SetTimerbyEvent (delegate Custom|UpdateProjectileCurve) 0.01 true))
  (Variables|Default|SetProjectileTimer _returnvalue))

(event Custom|UpdateProjectileCurve
  ;[0.15 0.07911 0.1459 0.5] Splines Throw Curve - Projected path
  (CallFunction|ClearSplines)
  (bind _returnvalue (CallFunction|ComputeThrowImpulse))
  (bind _predictresult (Class|GameplayStatics|BlueprintPredictProjectilePathAdvanced (Utilities|Struct|MakePredictProjectilePathParams (Transformation|GetWorldLocation (Variables|Default|GetThrowPoint)) _returnvalue true 0.0 1.0 true "ECC_WorldStatic" "ObjectTypeQuery1" (Utilities|Array|MakeArray self) 2e+01 0.0 "None" 5.0 false)))
  (for _array_element (.PathData (Utilities|Struct|BreakPredictProjectilePathResult _predictresult))
    (Spline|AddSplinePoint (Variables|Default|GetThrowSpline) (.Location (Utilities|Struct|BreakPredictProjectilePathPointData _array_element)) "World" true))
  (for _index (range 1 (Spline|GetNumberOfSplinePoints (Variables|Default|GetThrowSpline)))
    (bind _returnvalue_2 (AddComponent|AddSplineMeshComponent true))
    (Utilities|Array|Add (Variables|Default|GetSplineMesh) _returnvalue_2)
    (SplineMesh|SetStartandEnd _returnvalue_2 (.Location (Spline|GetLocationandTangentatSplinePoint (Variables|Default|GetThrowSpline) _index "World")) (.Tangent (Spline|GetLocationandTangentatSplinePoint (Variables|Default|GetThrowSpline) _index "World")) (Math|Vector|Lerp(Vector) (.Location (Spline|GetLocationandTangentatSplinePoint (Variables|Default|GetThrowSpline) _index "World")) (.Location (Spline|GetLocationandTangentatSplinePoint (Variables|Default|GetThrowSpline) (+ _index 1) "World")) 0.5) (Math|Vector|Lerp(Vector) (.Tangent (Spline|GetLocationandTangentatSplinePoint (Variables|Default|GetThrowSpline) _index "World")) (.Tangent (Spline|GetLocationandTangentatSplinePoint (Variables|Default|GetThrowSpline) (+ _index 1) "World")) 0.5) true :!class /Script/Engine.SplineMeshComponent)))

(event Custom|Clear_Splines
  (bind _splinemesh (Variables|Default|GetSplineMesh))
  ;[0.15 0.07911 0.1459 0.5] Splines Throw Curve - Projected path
  ;;[0.15 0.15 0.15 0.5] Clear Splines
  (Components|DestroyComponent _splinemesh)
  (Utilities|Array|Clear _splinemesh)
  (Spline|ClearSplinePoints (Variables|Default|GetThrowSpline) true))

(event Custom|Pickup_MC
  (params (In_Ball :type BP%20RHB%20Game%20Ball%20Object%20Reference))
  (bind _gameball (Variables|Default|GetgameBall))
  (bind _ballmesh (Variables|/Game/_RHB_MAIN/Blueprints/AActors/BP_RHB_GameBall.BP_RHB_GameBall_C|GetBallMesh In_Ball))
  ;[0.15 0.02353 0.01607 0.5] Pickup Custom Event
  (Physics|Components|PhysicsHandle|GrabComponentatLocationwithRotation (Variables|Default|GetPhysicsHandle) _ballmesh "None" (Transformation|GetWorldLocation _ballmesh) (Transformation|GetWorldRotation _ballmesh))
  (Variables|Default|SetbIsGrabbed true)
  (if (Utilities|IsValid _gameball)
    (Collision|SetActorEnableCollision _gameball false)
    (Collision|SetCollisionEnabled (Variables|/Game/_RHB_MAIN/Blueprints/AActors/BP_RHB_GameBall.BP_RHB_GameBall_C|GetBallMesh _gameball) "NoCollision")
    (CallFunction|Hold)))

(event Custom|Pickup_SV
  (params (Ball :type BP%20RHB%20Game%20Ball%20Object%20Reference))
  ;[0.15 0.02353 0.01607 0.5] Pickup Custom Event
  (CallFunction|PickupMC Ball))

(event Input|MouseEvents|DebugKeyLeftMouseButton
  (params (Key :type Key%20Structure :default "None") (ActionValue :type Input%20Action%20Value%20Structure))
  ;[0.15 0.03603 0.143 0.5] Throw Ball
  (:Pressed
    ;;[0.15 0.15 0.15 0.5] Wind-up Animation Montage
    (Animation|Montage|PlayMontage (Variables|Character|GetMesh) "/Game/_RHB_MAIN/Animations/OneHandLoop_Anim_Montage.OneHandLoop_Anim_Montage" 0.0
      (:then
        (CallFunction|DrawCurve))))
  (:Released
    ;;[0.15 0.15 0.15 0.5] Throw Montage
    (Animation|Montage|PlayMontage (Variables|Character|GetMesh) "/Game/_RHB_MAIN/Animations/OneHandEnd_Anim_Montage.OneHandEnd_Anim_Montage"
      (:OnNotifyBegin
        (Utilities|Time|ClearandInvalidateTimerbyHandle (Variables|Default|GetProjectileTimer))
        (CallFunction|ClearSplines)
        (bind _gameball (Variables|Default|GetgameBall)
          (:then
            (Collision|SetActorEnableCollision _gameball true)
            (Collision|SetCollisionEnabled (Variables|/Game/_RHB_MAIN/Blueprints/AActors/BP_RHB_GameBall.BP_RHB_GameBall_C|GetBallMesh _gameball) "QueryAndPhysics")
            (Physics|Components|PhysicsHandle|ReleaseComponent (Variables|Default|GetPhysicsHandle))
            (bind _returnvalue (CallFunction|ComputeThrowImpulse))
            (Physics|AddImpulse (Variables|/Game/_RHB_MAIN/Blueprints/AActors/BP_RHB_GameBall.BP_RHB_GameBall_C|GetBallMesh (Variables|Default|GetgameBall)) _returnvalue "None" true)
            (Transformation|SetActorRotation (Pawn|GetControlRotation :!class /Script/Engine.Pawn)))
          (:else))))))

(event Input|MouseEvents|DebugKeyRightMouseButton
  (params (Key :type Key%20Structure :default "None") (ActionValue :type Input%20Action%20Value%20Structure))
  ;[0.15 0.02353 0.01607 0.5] Pickup Custom Event
  (:Pressed
    (for _array_element (Collision|GetOverlappingActors (Variables|Default|GetPickupSphere) "/Game/_RHB_MAIN/Blueprints/AActors/BP_RHB_GameBall.BP_RHB_GameBall_C" :!class /Script/Engine.PrimitiveComponent)
      (bind _asbp_rhb_game_ball (Utilities|Casting|CastToBP_RHB_GameBall _array_element))
      (bind _output_get (Variables|Default|SetgameBall _asbp_rhb_game_ball))
      (CallFunction|PickupSV _output_get))))

(fn ConstructionScript)

(fn ComputeThrowImpulse
  (bind _followcamera (Variables|Default|GetFollowCamera))
  (bind _returnvalue (Transformation|GetWorldRotation _followcamera))
  (bind _returnvalue_2 (Math|Vector|GetForwardVector _returnvalue))
  (bind _returnvalue_3 (* _returnvalue_2 1e+03))
  (bind (_x _y) (Math|Vector|BreakVector _returnvalue_3))
  (return (Math|Vector|MakeVector _x _y (* (Math|Float|MapRangeClamped (.Z (Math|Vector|BreakVector _returnvalue_2)) 0.0 1.0 3.0 8.0) 1e+02))))