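; Interactable actor that recolors a fog mesh, a box mesh and a point light to a random color while the player is inside its collision box.
; Both the interface OnInteract event and the first-person character's PressE dispatcher, bound at BeginPlay, run the same color change.
; Dynamic material instances for fog, box and button receive parameter changes, with interaction also resetting the button's State and hiding the PressE prompt.
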(event OnComponentBeginOverlap(Collision)
  (params (OtherActor :type Actor%20Object%20Reference) (OtherComp :type Primitive%20Component%20Object%20Reference) (OtherBodyIndex :type Integer) (bFromSweep :type Boolean) (SweepResult :type Hit%20Result%20Structure%20%28by%20ref%29))
  ;[1 1 1] Can only interact with BP if overlapping collision box
  (Utilities|Casting|CastToFirstPersonCharacter OtherActor)
  (Variables|Default|SetisOverlapping true))

(event OnComponentEndOverlap(Collision)
  (params (OtherActor :type Actor%20Object%20Reference) (OtherComp :type Primitive%20Component%20Object%20Reference) (OtherBodyIndex :type Integer))
  ;[1 1 1] Can only interact with BP if overlapping collision box
  (Utilities|Casting|CastToFirstPersonCharacter OtherActor)
  (Variables|Default|SetisOverlapping false))

(event Custom|Interact
  ;[1 1 1] Top - Blueprint Interface (raycast right click), Bottom - Dispatcher Custom event (Press 'E' key)
  (if (Variables|Default|GetisOverlapping)
    (Rendering|Material|SetScalarParameterValue (Variables|Default|GetButton_DMI) "State" 0.0 :!class /Script/Engine.MaterialInstanceDynamic)
    (Rendering|SetVisibility (Variables|Default|GetPress%20E%20) false false)
    (Variables|Default|SetSetColor (Utilities|Struct|MakeLinearColor (Math|Random|RandomFloatinRange 0.0 0.8) (Math|Random|RandomFloatinRange 0.0 0.8) (Math|Random|RandomFloatinRange 0.0 0.8) 0.0))
    ;;[1 1 1] Sets color of newly created Dynamic Material to the random color variable that was just created.  Also sets the point color to the same thing.
    (Rendering|Material|SetVectorParameterValue (Variables|Default|GetDMI_Fog) "Color" (Variables|Default|GetSetColor) :!class /Script/Engine.MaterialInstanceDynamic)
    (Rendering|Material|SetVectorParameterValue (Variables|Default|GetDMI_Box) "DiffuseColor" (Variables|Default|GetSetColor) :!class /Script/Engine.MaterialInstanceDynamic)
    (Rendering|Components|Light|SetLightColor (Variables|Default|GetPointLight) (Variables|Default|GetSetColor) false)))

(event EventBeginPlay
  ;[1 1 1] Begin Play - Sets up Dynamic Materials for 2 Materials and sets them to variables to be manipulated.  Also Casts to FPCharacter in order to bind the 'E' key dispatcher to a custom event
  (bind _returnvalue (Rendering|Material|CreateDynamicMaterialInstance (Variables|Default|GetfogMesh) 0 (Rendering|Material|GetMaterial (Variables|Default|GetfogMesh) 0) :!class /Script/Engine.PrimitiveComponent))
  (Variables|Default|SetDMI_Fog _returnvalue)
  (bind _returnvalue_2 (Rendering|Material|CreateDynamicMaterialInstance (Variables|Debug|GetStaticMeshComponent) 0 (Rendering|Material|GetMaterial (Variables|Debug|GetStaticMeshComponent) 0) :!class /Script/Engine.PrimitiveComponent))
  (Variables|Default|SetDMI_Box _returnvalue_2)
  (bind _asfirst_person_character (Utilities|Casting|CastToFirstPersonCharacter (Game|GetPlayerCharacter 0)))
  (EventDispatchers|BindEventtoPressEDispatcher _asfirst_person_character (delegate Custom|Interact)))

(event EventOnInteract
  ;[1 1 1] Top - Blueprint Interface (raycast right click), Bottom - Dispatcher Custom event (Press 'E' key)
  (if (Variables|Default|GetisOverlapping)
    (Rendering|Material|SetScalarParameterValue (Variables|Default|GetButton_DMI) "State" 0.0 :!class /Script/Engine.MaterialInstanceDynamic)
    (Rendering|SetVisibility (Variables|Default|GetPress%20E%20) false false)
    (Variables|Default|SetSetColor (Utilities|Struct|MakeLinearColor (Math|Random|RandomFloatinRange 0.0 0.8) (Math|Random|RandomFloatinRange 0.0 0.8) (Math|Random|RandomFloatinRange 0.0 0.8) 0.0))
    ;;[1 1 1] Sets color of newly created Dynamic Material to the random color variable that was just created.  Also sets the point color to the same thing.
    (Rendering|Material|SetVectorParameterValue (Variables|Default|GetDMI_Fog) "Color" (Variables|Default|GetSetColor) :!class /Script/Engine.MaterialInstanceDynamic)
    (Rendering|Material|SetVectorParameterValue (Variables|Default|GetDMI_Box) "DiffuseColor" (Variables|Default|GetSetColor) :!class /Script/Engine.MaterialInstanceDynamic)
    (Rendering|Components|Light|SetLightColor (Variables|Default|GetPointLight) (Variables|Default|GetSetColor) false)))

(fn ConstructionScript
  (bind _returnvalue (Rendering|Material|CreateDynamicMaterialInstance (Variables|Default|GetButton) 2 "/Game/DemoRoom/Materials/M_Button_Inst.M_Button_Inst" :!class /Script/Engine.PrimitiveComponent))
  (Variables|Default|SetButton_DMI _returnvalue))