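; Chair actor that moves up when shot and down when interacted with, hiding a text prompt each time.
; A hit from a FirstPersonProjectile plays the MoveUp timeline, while OnInteract, commented as a right-click raycast, plays MoveDown.
; Both timelines offset the actor from CurrentLocation, which Tick refreshes every frame, so offsets accumulate during playback rather than measuring from a fixed start.
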(event EventTick
  (params (DeltaSeconds :type Float%20%28single-precision%29))
  ;[1 1 1] Get current location
  (Variables|Default|SetCurrentLocation (Transformation|GetActorLocation)))

(event Collision|EventHit
  (params (MyComp :type Primitive%20Component%20Object%20Reference) (Other :type Actor%20Object%20Reference) (OtherComp :type Primitive%20Component%20Object%20Reference) (bSelfMoved :type Boolean) (HitLocation :type Vector :default "0, 0, 0") (HitNormal :type Vector :default "0, 0, 0") (NormalImpulse :type Vector :default "0, 0, 0") (Hit :type Hit%20Result%20Structure%20%28by%20ref%29))
  ;[1 1 1] Shoot to Move up
  (Utilities|Casting|CastToFirstPersonProjectile Other)
  (Rendering|SetVisibility (Variables|Default|GetShootMeText) false false)
  (bind _moveup (Timeline|MoveUp PlayFromStart)
    (:Update
      (Transformation|SetActorLocation (+ (Variables|Default|GetCurrentLocation) _moveup) false false))))

(event EventOnInteract
  ;[1 1 1] RayCast (right click) to Move Down
  (Rendering|SetVisibility (Variables|Default|GetTextRender2) false false)
  (bind _down (Timeline|MoveDown PlayFromStart)
    (:Update
      (Transformation|SetActorLocation (- (Variables|Default|GetCurrentLocation) _down) false false))))

(fn ConstructionScript)