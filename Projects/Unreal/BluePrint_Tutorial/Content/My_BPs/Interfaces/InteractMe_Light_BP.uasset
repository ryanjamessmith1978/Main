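; Interactable light Blueprint that changes to a random color when the player or another caller triggers its OnInteract event.
; OnInteract calls ChangeLightColor, which gives the SpotLight and PointLight random RGB colors, then hides the Raycasttext component.
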(event Custom|Change%20Light%20Color
  (Rendering|Components|Light|SetLightColor (Variables|Default|GetSpotLight) (Utilities|Struct|MakeLinearColor (Math|Random|RandomFloatinRange 0.0 1.0) (Math|Random|RandomFloatinRange 0.0 1.0) (Math|Random|RandomFloatinRange 0.0 1.0) 0.0) true))

(event EventOnInteract
  (CallFunction|ChangeLightColor)
  (Rendering|SetVisibility (Variables|Default|Getraycasttext) false false))

(fn ConstructionScript)