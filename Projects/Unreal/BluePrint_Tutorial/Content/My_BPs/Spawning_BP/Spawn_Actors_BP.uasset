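; An interactable spawner actor with a switch that starts an endless stream of randomly rotated Box_for_Spawner_BP actors at its location.
; It binds to the first-person character's press-E dispatcher and responds only while that character overlaps its collision volume.
; Activation hides the prompt text, sets the button's dynamic material state, spawns immediately and starts a looping timer.
; The timer's interval is randomized once per activation, and nothing in this Blueprint stops it.
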(event OnComponentBeginOverlap(CollisionVolume)
  (params (OtherActor :type Actor%20Object%20Reference) (OtherComp :type Primitive%20Component%20Object%20Reference) (OtherBodyIndex :type Integer) (bFromSweep :type Boolean) (SweepResult :type Hit%20Result%20Structure%20%28by%20ref%29))
  ;[1 1 1] Sets Overlapping Bool ean
  (Utilities|Casting|CastToFirstPersonCharacter OtherActor)
  (Variables|Default|SetisOverlappingCollision true))

(event OnComponentEndOverlap(CollisionVolume)
  (params (OtherActor :type Actor%20Object%20Reference) (OtherComp :type Primitive%20Component%20Object%20Reference) (OtherBodyIndex :type Integer))
  ;[1 1 1] Sets Overlapping Bool ean
  (Utilities|Casting|CastToFirstPersonCharacter OtherActor)
  (Variables|Default|SetisOverlappingCollision false))

(event Custom|StartSpawn
  ;[1 1 1] Starts Spawning Loop based on overlap
  (if (Variables|Default|GetisOverlappingCollision)
    (Rendering|SetVisibility (Variables|Default|GetTextRendera%20) false false)
    (Rendering|Material|SetScalarParameterValue (Variables|Default|GetCreateDMI) "State" 0.0 :!class /Script/Engine.MaterialInstanceDynamic)
    (CallFunction|SpawnActors)
    (Utilities|Time|SetTimerbyFunctionName self "SpawnActors" (Math|Random|RandomFloatinRange 0.5 1.5) true)))

(event Custom|SpawnActors
  ;[1 1 1] Custom Event that Spawns the Actual Actor
  (Game|SpawnActorfromClass "/Game/My_BPs/Spawning_BP/box_for_Spawner_BP.box_for_Spawner_BP_C" (Math|Transform|MakeTransform (Transformation|GetActorLocation) (Math|Random|RandomRotator false) "1,1,1") "Undefined" 0 0))

(event EventBeginPlay
  ;[1 1 1] Begin Play - Creates Dispatcher (allows for E to be used to activate this BP
  (bind _asfirst_person_character (Utilities|Casting|CastToFirstPersonCharacter (Game|GetPlayerCharacter 0)))
  (bind _output_get (Variables|Default|SetMyCharacter _asfirst_person_character))
  (EventDispatchers|BindEventtoPressEDispatcher _output_get (delegate Custom|StartSpawn)))

(fn ConstructionScript
  (Transformation|SetRelativeScale3D (Variables|Default|Getswitch) "0.750000,0.750000,0.750000")
  (Transformation|SetRelativeScale3D (Variables|Default|GetblockPile) "1.500000,1.500000,1.500000")
  (bind _returnvalue (Rendering|Material|CreateDynamicMaterialInstance (Variables|Default|Getswitch) 2 "/Game/DemoRoom/Materials/M_Button_Inst.M_Button_Inst" :!class /Script/Engine.PrimitiveComponent))
  (Variables|Default|SetCreateDMI _returnvalue))