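; MyConveyer_Volume_BP is a conveyor belt volume that carries overlapping actors along its forward direction.
; Each tick it offsets every overlapping actor by its forward vector, scaled by Speed and delta time, without sweep or class filtering.
; An Arrow rescale that would cancel the actor's scale sits unconnected, so the construction script does nothing.
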(event EventTick
  (params (DeltaSeconds :type Float%20%28single-precision%29))
  (for _array_element (Collision|GetOverlappingActors 0 :!class /Script/Engine.Actor)
    (Transformation|AddActorWorldOffset _array_element (* (Math|Vector|GetForwardVector (Transformation|GetActorRotation)) (* DeltaSeconds (Variables|Default|GetSpeed))))))

(fn ConstructionScript)