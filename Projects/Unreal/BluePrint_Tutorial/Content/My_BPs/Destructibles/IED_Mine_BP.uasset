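; IED_Mine_BP is a one-shot mine that explodes when hit by a FirstPersonCharacter.
; A cast filters the Hit event and a DoOnce keeps it from triggering again.
; On trigger it launches the character upward, spawns an explosion emitter, activates its RadialForce component and plays a sound at its location.
; The actor destroys itself after a short delay.
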(event Collision|EventHit
  (params (MyComp :type Primitive%20Component%20Object%20Reference) (Other :type Actor%20Object%20Reference) (OtherComp :type Primitive%20Component%20Object%20Reference) (bSelfMoved :type Boolean) (HitLocation :type Vector :default "0, 0, 0") (HitNormal :type Vector :default "0, 0, 0") (NormalImpulse :type Vector :default "0, 0, 0") (Hit :type Hit%20Result%20Structure%20%28by%20ref%29))
  (bind _asfirst_person_character (Utilities|Casting|CastToFirstPersonCharacter Other))
  (Utilities|FlowControl|DoOnce false
    (:Completed
      (Character|LaunchCharacter _asfirst_person_character "0, 0,1000.000000" false false)
      (Effects|SpawnEmitteratLocation "/Game/StarterContent/Particles/P_Explosion.P_Explosion" (Transformation|GetActorLocation))
      (Components|Activation|Activate (Variables|Default|GetRadialForce) false)
      (Audio|PlaySoundatLocation "/Game/StarterContent/Audio/Explosion01.Explosion01" (Transformation|GetActorLocation) "0, 0, 0" 0.6)
      (Utilities|FlowControl|Delay 3.0)
      (Actor|DestroyActor))))

(fn ConstructionScript)