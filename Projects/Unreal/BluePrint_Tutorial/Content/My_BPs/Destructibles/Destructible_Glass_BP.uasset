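; Destructible glass actor that responds to first-person projectile hits with a breaking sound and slow-motion shatter.
; A hit from a FirstPersonProjectile plays a 2D glass-breaking sound and enables physics simulation on its DestructibleComponent.
; When the component fractures, it issues a slomo console command for half speed, then after a delay issues one for normal speed and destroys the actor.
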(event OnComponentFracture(DestructibleComponent)
  (params (HitPoint :type Vector%20%28by%20ref%29) (HitDirection :type Vector%20%28by%20ref%29 :default "0, 0, 0"))
  (Development|ExecuteConsoleCommand (Utilities|String|BuildString(Float) "" "slomo " 0.5))
  (Utilities|FlowControl|Delay 2.5)
  (Development|ExecuteConsoleCommand (Utilities|String|BuildString(Float) "" "slomo " 1.0))
  (Actor|DestroyActor))

(event Collision|EventHit
  (params (MyComp :type Primitive%20Component%20Object%20Reference) (Other :type Actor%20Object%20Reference) (OtherComp :type Primitive%20Component%20Object%20Reference) (bSelfMoved :type Boolean) (HitLocation :type Vector :default "0, 0, 0") (HitNormal :type Vector :default "0, 0, 0") (NormalImpulse :type Vector :default "0, 0, 0") (Hit :type Hit%20Result%20Structure%20%28by%20ref%29))
  (Utilities|Casting|CastToFirstPersonProjectile Other)
  (Audio|SpawnSound2D "/Game/FirstPerson/Audio/159197__justbrando__glass-breaking_1.159197__justbrando__glass-breaking_1")
  (Physics|SetSimulatePhysics (Variables|Default|GetDestructibleComponent) true))

(fn ConstructionScript)