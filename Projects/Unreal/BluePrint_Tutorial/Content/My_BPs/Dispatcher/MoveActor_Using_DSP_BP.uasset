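; Actor Blueprint that demonstrates an Event Dispatcher by announcing when it is hit and exposing a way to move its mesh.
; Hit calls the YouHitMeED dispatcher, while the MoveMesh custom event offsets the static mesh along local Z by a given amount, intended for Level Blueprint use.
; A RotateMesh timeline, noted as auto-start with no execution input, lerps yaw through 360 degrees from the rotation cached at BeginPlay.
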(event Custom|MoveMesh
  (params (Amount :type Float%20%28single-precision%29))
  ;[1 1 1] Custom Event that can be called from the Level BP if <this class> is referenced in the level.  Call Move Mesh Function, and it can be fired by using the event dispatcher Event
  (Transformation|AddLocalOffset (Variables|Default|GetStaticMesh) (Math|Vector|MakeVector 0.0 0.0 Amount) false false))

(event Collision|EventHit
  (params (MyComp :type Primitive%20Component%20Object%20Reference) (Other :type Actor%20Object%20Reference) (OtherComp :type Primitive%20Component%20Object%20Reference) (bSelfMoved :type Boolean) (HitLocation :type Vector :default "0, 0, 0") (HitNormal :type Vector :default "0, 0, 0") (NormalImpulse :type Vector :default "0, 0, 0") (Hit :type Hit%20Result%20Structure%20%28by%20ref%29))
  ;[1 1 1] Sets up an Event Dispatcher with Call Dispatcher to fire when object is hit
  (Default|CallYouHitMeED))

(event EventBeginPlay
  ;[1 1 1] Begin Play - Sets Initial Rotation
  (Variables|Default|SetActorCurrentRot (Transformation|GetActorRotation)))

(fn ConstructionScript)