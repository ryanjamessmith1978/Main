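; Flashy_BP is a trigger-activated light that flashes with sound while the player is inside its volume.
; When FirstPersonCharacter begins overlapping Trigger, it shows the PointLight, plays an audio clip assigned at BeginPlay, and starts a timeline that drives the light's intensity.
; On end overlap it stops the audio and hides the light, but leaves the timeline running.
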(event OnComponentBeginOverlap(Trigger)
  (params (OtherActor :type Actor%20Object%20Reference) (OtherComp :type Primitive%20Component%20Object%20Reference) (OtherBodyIndex :type Integer) (bFromSweep :type Boolean) (SweepResult :type Hit%20Result%20Structure%20%28by%20ref%29))
  (Utilities|Casting|CastToFirstPersonCharacter OtherActor)
  (Audio|Components|Audio|Play (Variables|Default|GetAudio_Flashy_Sound) 0.0)
  (Rendering|SetVisibility (Variables|Default|GetPointLight) true false)
  (bind _brightness (Timeline|Timeline_0 Play)
    (:Update
      (Rendering|Components|Light|SetIntensity (Variables|Default|GetPointLight) _brightness))))

(event OnComponentEndOverlap(Trigger)
  (params (OtherActor :type Actor%20Object%20Reference) (OtherComp :type Primitive%20Component%20Object%20Reference) (OtherBodyIndex :type Integer))
  (Utilities|Casting|CastToFirstPersonCharacter OtherActor)
  (Audio|Components|Audio|Stop (Variables|Default|GetAudio_Flashy_Sound))
  (Rendering|SetVisibility (Variables|Default|GetPointLight) false false))

(event EventBeginPlay
  (Audio|Components|Audio|SetSound (Variables|Default|GetAudio_Flashy_Sound) "/Game/My_BPs/Audio/263621__jamesabdulrahman__permission-to-panic.263621__jamesabdulrahman__permission-to-panic"))

(fn ConstructionScript)