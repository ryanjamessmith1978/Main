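; Interactive door actor that swings 90 degrees open or closed with a sound when the first-person player presses E nearby.
; BeginPlay stores the starting rotation and binds OpenDoor to the character's Press E dispatcher.
; A Box trigger gates input and toggles the tip's visibility; an accepted press hides the tip in game.
; OpenDoor flips DoorOpen and plays or reverses the Rotate timeline, which lerps yaw from the stored rotation.
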(event OnComponentBeginOverlap(Box)
  (params (OverlappedComponent :type Primitive%20Component%20Object%20Reference) (OtherActor :type Actor%20Object%20Reference) (OtherComp :type Primitive%20Component%20Object%20Reference) (OtherBodyIndex :type Integer) (bFromSweep :type Boolean) (SweepResult :type Hit%20Result%20Structure%20%28by%20ref%29))
  ;[1 0.3828 0.6604] Trigger enables and disables Player Input as well as the Helpful Tip
  (Utilities|Casting|CastToFirstPersonCharacter OtherActor)
  (Variables|Default|SetInputEnabled true)
  (Rendering|SetVisibility (Variables|Default|GetHelpful_tip%20) true false))

(event OnComponentEndOverlap(Box)
  (params (OverlappedComponent :type Primitive%20Component%20Object%20Reference) (OtherActor :type Actor%20Object%20Reference) (OtherComp :type Primitive%20Component%20Object%20Reference) (OtherBodyIndex :type Integer))
  ;[1 0.3828 0.6604] Trigger enables and disables Player Input as well as the Helpful Tip
  (Utilities|Casting|CastToFirstPersonCharacter OtherActor)
  (Variables|Default|SetInputEnabled false)
  (Rendering|SetVisibility (Variables|Default|GetHelpful_tip%20) false false))

(event Custom|OpenDoor
  (bind _current_actor_rotation (Variables|Default|GetCurrent%20Actor%20rotation))
  (bind (_roll _pitch _yaw) (Math|Rotator|BreakRotator _current_actor_rotation))
  ;[1 1 1] Pressing E erases on Screen Text tip, and switches door open boolean
  (if (Variables|Default|GetInputEnabled)
    (Development|SetHiddeninGame (Variables|Default|GetHelpful_tip%20) true false)
    (if (Variables|Default|GetDoorOpen)
      (Variables|Default|SetDoorOpen false)
      (Audio|PlaySoundatLocation "/Game/My_BPs/Audio/344360__amholma__door-open-close___1.344360__amholma__door-open-close___1" (Transformation|GetActorLocation))
      ;[1 1 1] Set rotation of the Door using a Timeline and LERP (Linear Interpolation)
      (bind _rotatedoor (Timeline|rotate Reverse)
        (:Update
          (Transformation|SetActorRotation (Math|Rotator|MakeRotator _roll _pitch (Math|Float|Lerp _yaw (+ (.Yaw (Math|Rotator|BreakRotator _current_actor_rotation)) 9e+01) _rotatedoor)))))
      (else
        (Variables|Default|SetDoorOpen true)
        (Audio|PlaySoundatLocation "/Game/My_BPs/Audio/Door_Open.Door_Open" (Transformation|GetActorLocation))
        (Timeline|rotate Play)))))

(event EventBeginPlay
  ;[1 1 1] Event Play - sets Door Rotation, cast to Player Character to bind event 'Press E'
  (Variables|Default|SetCurrent%20Actor%20rotation (Transformation|GetActorRotation))
  (bind _asfirst_person_character (Utilities|Casting|CastToFirstPersonCharacter (Game|GetPlayerCharacter 0)))
  (bind _output_get (Variables|Default|SetMyChar _asfirst_person_character))
  (EventDispatchers|BindEventtoPressEDispatcher _output_get (delegate Custom|OpenDoor)))

(fn ConstructionScript)