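; BP_GameBall is a physics ball actor that can be thrown from the player's third-person character.
; BeginPlay caches the player's BP_ThirdPersonCharacter.
; Throw applies an impulse to the ball's static mesh along the forward vector of the character mesh's "ball" socket, at that socket's location.
; The Hit event is empty, and logic to push simulating components by the ball's velocity is left disconnected.
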(event Custom|Throw
  (bind _as_bp_third_person_character (Variables|Default|GetAs%20BP%20Third%20Person%20Character))
  (bind _mesh (Variables|/Script/Engine.Character|GetMesh _as_bp_third_person_character))
  (Physics|AddImpulseatLocation (Variables|Debug|GetStaticMeshComponent) (* (Math|Vector|GetForwardVector (Transformation|GetSocketRotation _mesh "ball")) 5e+01) (Transformation|GetSocketLocation _mesh "ball") "ball"))

(event EventBeginPlay
  (bind _asbp_third_person_character (Utilities|Casting|CastToBP_ThirdPersonCharacter (Game|GetPlayerCharacter 0)))
  (Variables|Default|SetAs%20BP%20Third%20Person%20Character _asbp_third_person_character))

(event Collision|EventActorBeginOverlap
  (params (OtherActor :type Actor%20Object%20Reference)))

(event EventTick
  (params (DeltaSeconds :type Float%20%28single-precision%29)))

(event Collision|EventHit
  (params (MyComp :type Primitive%20Component%20Object%20Reference) (Other :type Actor%20Object%20Reference) (OtherComp :type Primitive%20Component%20Object%20Reference) (bSelfMoved :type Boolean) (HitLocation :type Vector :default "0, 0, 0") (HitNormal :type Vector :default "0, 0, 0") (NormalImpulse :type Vector :default "0, 0, 0") (Hit :type Hit%20Result%20Structure%20%28by%20ref%29)))

(fn ConstructionScript)