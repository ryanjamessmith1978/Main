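; BP_RobotGameState is a game state Blueprint meant to track two players' scores, though its scoring logic is currently disconnected.
; On BeginPlay it casts the game mode to BP_RobotHead_GM and caches it along with its MainGUI reference.
; AddToScore and AddToScoreRPC are empty; orphaned nodes hold the logic to increment Player1Score or Player2Score and update the GUI score text.
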(event Custom|AddToScore
  (params (WhichPlayer :type Integer)))

(event Custom|AddToScoreRPC)

(event EventBeginPlay
  (bind _asbp_robot_head_gm (Utilities|Casting|CastToBP_RobotHead_GM (Game|GetGameMode)))
  (bind _output_get (Variables|Default|SetAs%20BP%20Robot%20Head%20GM _asbp_robot_head_gm))
  (Variables|Default|SetMain%20GUI (Variables|/Game/_MyStuff/Blueprints/Core/BP_RobotHead_GM.BP_RobotHead_GM_C|GetMainGUI _output_get)))

(event EventTick
  (params (DeltaSeconds :type Float%20%28single-precision%29)))

(fn ConstructionScript)