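; Main game mode that numbers joining players and spawns the game ball for a multiplayer match.
; On PostLogin it increments a joined-player counter and passes that ID through an RPC-named event to SetUniqueID on the player's BP_RobotHead_PC.
; Once at least two players have joined, each login spawns a BP_GameBall at the spawn point and stores it as BallSpawned.
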(event Custom|UniqueID_RPC
  (params (PC :type Player%20Controller%20Object%20Reference) (playerID :type Integer))
  (CallFunction|UniqueID PC playerID))

(event Custom|UniqueID
  (params (PlayerControl :type Player%20Controller%20Object%20Reference) (PlayerID :type Integer))
  (bind _asbp_robot_head_pc (Utilities|Casting|CastToBP_RobotHead_PC PlayerControl))
  (Default|SetUniqueID _asbp_robot_head_pc PlayerID))

(event EventBeginPlay)

(event EventPostLogin
  (params (NewPlayer :type Player%20Controller%20Object%20Reference))
  (bind _result (Math|Integer|IncrementInt (Variables|Default|GetnunPlayersJoined))
    (:%20%20
      (CallFunction|UniqueIDRPC NewPlayer _result)
      (if (>= (Variables|Default|GetnunPlayersJoined) 2)
        (bind _returnvalue (Game|SpawnActorfromClass "/Game/_MyStuff/Blueprints/AActors/BP_GameBall.BP_GameBall_C" (Math|Transform|MakeTransform (Variables|Default|GetSpawnPoint) "0, 0, 0" "1.000000,1.000000,1.000000") "Undefined" "MultiplyWithRoot" (Components|GetOwner) 0 0))
        (Variables|Default|SetBallSpawned _returnvalue)))))

(fn ConstructionScript)