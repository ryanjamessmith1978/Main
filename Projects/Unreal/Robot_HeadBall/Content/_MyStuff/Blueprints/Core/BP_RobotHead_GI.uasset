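; BP_RobotHead_GI is the game instance Blueprint that handles online session matchmaking with a join-or-host flow.
; JoinMatch searches for sessions and joins the first result, calls CreateSession when none are found, and prints a message if the search fails.
; CreateSession starts an async two-player session and opens MainArena as a listen server from the task's immediate Then output, without waiting for success.
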(event Custom|CreateSession
  ;[0.15 0.15 0.15 0.5] ASync Task
  (|Session (Game|GetPlayerController 0) 2 false true
    (:then
      (Game|OpenLevel(byName) "MainArena" true "listen"))))

(event Custom|JoinMatch
  (bind _results (|FindSessions (Game|GetPlayerController 0) 100 false false)
    (:OnSuccess
      (if (> (Utilities|Array|Length _results) 0)
        (|JoinSession (Game|GetPlayerController 0) (Utilities|Array|Get(acopy) _results))
        (else
          (CallFunction|CreateSession))))
    (:OnFailure
      (Development|PrintString "Failsure"))))