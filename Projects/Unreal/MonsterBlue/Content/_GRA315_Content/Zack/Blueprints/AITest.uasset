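; AI character for a level-based game that reacts to overlapping hazards, bonus items and the exit, tracking tries, bonuses and score.
; It caches its starting transform on BeginPlay, then teleports back there and counts a try after hitting a Hazard.
; Touching an EndPoint marks the level finished and adds score.
; A BonusItem is destroyed on overlap, then counted and scored after a brief delay.
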(event Collision|EventActorBeginOverlap
  (params (OtherActor :type Actor%20Object%20Reference))
  ;[1 1 1] Reset AI Pos/Rot after hitting a hazard
  (Utilities|Casting|CastToHazard OtherActor
    (:then
      (Components|Movement|StopMovementImmediately (Variables|Character|GetCharacterMovement))
      (Transformation|Teleport (Variables|Default|GetStartPos) (Variables|Default|GetStartRot))
      (Utilities|FlowControl|Delay 0.2)
      (CallFunction|IncreaseTries))
    (:CastFailed
      ;[1 1 1] Set LevelFinished to True when the AI hits the exit
      (Utilities|Casting|CastToEndPoint OtherActor
        (:then
          (Variables|Default|SetLevelFinished true)
          (Variables|Default|SetScore (+ (Variables|Default|GetScore) 1000)))
        (:CastFailed
          ;[1 1 1] Add bonus when collected (and destroy the collectible)
          (bind _asbonus_item (Utilities|Casting|CastToBonusItem OtherActor))
          (Actor|DestroyActor _asbonus_item)
          (Utilities|FlowControl|Delay 0.2)
          (CallFunction|IncreaseBonuses)
          (Variables|Default|SetScore (+ (Variables|Default|GetScore) 150)))))))

(event EventBeginPlay
  ;[1 1 1] Set AI Start Pos/Rot
  (Variables|Default|SetStartPos (Transformation|GetActorLocation))
  (Variables|Default|SetStartRot (Transformation|GetActorRotation)))

(fn ConstructionScript)

(fn IncreaseTries
  (bind _result (Math|Integer|IncrementInt (Variables|Default|GetNumTries))
    (:%20%20
      (Variables|Default|SetNumTries _result))))

(fn IncreaseBonuses
  (bind _result (Math|Integer|IncrementInt (Variables|Default|GetNumBonuses))
    (:%20%20
      (Variables|Default|SetNumBonuses _result))))