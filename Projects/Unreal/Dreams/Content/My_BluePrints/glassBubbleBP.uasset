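; Glass bubble Blueprint containing an unused yaw-spin animation, with nothing happening at BeginPlay.
; The construction script stores the actor's starting rotation and location, though only the rotation is read.
; An unconnected Rotate timeline would lerp yaw through a full turn from the stored rotation.
; Its Finished pin feeds back into a FlipFlop that alternates forward and reverse playback, but no event triggers this chain.
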(event EventBeginPlay)

(fn ConstructionScript
  (Variables|Default|SetstartingRotation (Transformation|GetActorRotation))
  (Variables|Default|SetstartingLocation (Transformation|GetActorLocation)))