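; Blueprint function library of small math and utility helpers for the MobileNavigation system.
; Screen helpers normalize a 2D value against a player's viewport size, clamped to 0–1 per axis.
; Vector helpers cover per-axis FInterpTo smoothing, component-wise 2D multiplication, 2D and 3D distance, and offsetting a location along a direction.
; A class check reports whether an actor's class derives from a given class.
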(fn ScalebyScreenSize
  (params (Unscaled :type Vector%202D%20Structure) (Player%20Index :type Integer))
  (bind _returnvalue (Game|GetPlayerController Player%20Index))
  (bind (_sizex _sizey) (HUD|GetViewportSize _returnvalue))
  (return (Math|Vector2D|MakeVector2D (Math|Float|Clamp(Float) (/ (.x Unscaled) (Math|Conversions|ToFloat(Integer) _sizex))) (Math|Float|Clamp(Float) (/ (.y Unscaled) (Math|Conversions|ToFloat(Integer) _sizey))))))

(fn Vector2DInterp
  (params (Current :type Vector%202D%20Structure) (Target :type Vector%202D%20Structure) (Speed :type Float%20%28single-precision%29) (DeltaTime :type Float%20%28single-precision%29))
  (return (Math|Vector2D|MakeVector2D (Math|Interpolation|FInterpTo (.x Current) (.x Target) DeltaTime Speed) (Math|Interpolation|FInterpTo (.y Current) (.y Target) DeltaTime Speed))))

(fn Vector2D*Vector2D
  (params (A :type Vector%202D%20Structure) (B :type Vector%202D%20Structure))
  (bind (_x _y) (Math|Vector2D|BreakVector2D B))
  (bind (_x_2 _y_2) (Math|Vector2D|BreakVector2D A))
  (return (Math|Vector2D|MakeVector2D (* _x_2 _x) (* _y_2 _y))))

(fn DistanceBetween
  (params (A :type Vector) (B :type Vector))
  (return (Math|Vector|VectorLength (- A B))))

(fn DistanceBetween(Vector2D)
  (params (A :type Vector%202D%20Structure) (B :type Vector%202D%20Structure))
  (return (Math|Vector2D|Vector2DLength (- A B))))

(fn OffsetinDirection
  (params (Location :type Vector) (Direction :type Vector) (Offset :type Float%20%28single-precision%29))
  (return (+ Location (* Direction Offset))))

(fn IsClassOf
  (params (Actor :type Actor%20Object%20Reference) (Class :type Actor%20Class%20Reference))
  (return (Utilities|ClassIsChildOf (Utilities|GetClass Actor) Class)))