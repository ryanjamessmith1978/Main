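; HUD for mobile navigation that shows tap-to-move feedback, either through UMG or by drawing directly on the HUD.
; The UseUMGHud macro branches on UseUMG: when true, BeginPlay adds a widget to the viewport.
; Otherwise, TapToMoveStart restarts the TapScale timeline and DrawHUD draws the joystick background texture at the tap position.
; The timeline drives size and opacity, with placement computed relative to screen width.
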(event Custom|Tap%20To%20Move%20Start
  (params (X :type Float%20%28single-precision%29) (Y :type Float%20%28single-precision%29))
  ;[1 1 1] Draw Tap to Move
  (Utilities|UseUMGHud
    (:False
      (bind _scale (Timeline|Tap%20Scale PlayFromStart)))))

(event Custom|Draw%20Tap%20To%20Move
  (params (SizeX :type Float%20%28single-precision%29))
  ;[1 1 1] Draw Tap to Move
  (Canvas|DrawTexture "/Engine/MobileResources/HUD/VirtualJoystick_Background.VirtualJoystick_Background" (.Out%20X (CallFunction|RelativePosandSizewithOffset SizeX (stale Custom|Tap%20To%20Move%20Start X) (stale Custom|Tap%20To%20Move%20Start Y) (* (stale Custom|Tap%20To%20Move%20Start _scale) 1.2e+02) 0.5 0.5)) (.Out%20Y (CallFunction|RelativePosandSizewithOffset SizeX (stale Custom|Tap%20To%20Move%20Start X) (stale Custom|Tap%20To%20Move%20Start Y) (* (stale Custom|Tap%20To%20Move%20Start _scale) 1.2e+02) 0.5 0.5)) (.Out%20Size (CallFunction|RelativePosandSizewithOffset SizeX (stale Custom|Tap%20To%20Move%20Start X) (stale Custom|Tap%20To%20Move%20Start Y) (* (stale Custom|Tap%20To%20Move%20Start _scale) 1.2e+02) 0.5 0.5)) (.Out%20Size (CallFunction|RelativePosandSizewithOffset SizeX (stale Custom|Tap%20To%20Move%20Start X) (stale Custom|Tap%20To%20Move%20Start Y) (* (stale Custom|Tap%20To%20Move%20Start _scale) 1.2e+02) 0.5 0.5)) 0.0 0.0 1.0 1.0 (Utilities|Struct|MakeLinearColor 1.0 1.0 1.0 (stale Custom|Tap%20To%20Move%20Start _scale)) "BLEND_Translucent" 1.0 true))

(event EventBeginPlay
  ;[1 1 1] Init
  (Utilities|UseUMGHud
    (:True
      (bind _returnvalue (Class|WidgetBlueprintLibrary|Create 0 (Game|Player|GetOwningPlayerController)))
      (UserInterface|Viewport|AddtoViewport _returnvalue))))

(event EventDrawHUD
  (params (SizeX :type Integer) (SizeY :type Integer))
  ;[1 1 1] Init
  (Utilities|UseUMGHud
    (:False
      (CallFunction|DrawTaptoMove (Math|Conversions|ToFloat(Integer) SizeX)))))

(fn ConstructionScript)