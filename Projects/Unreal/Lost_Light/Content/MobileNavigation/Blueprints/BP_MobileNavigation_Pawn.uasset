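; Mobile navigation pawn that provides swipe-to-look and tap-to-move touch controls.
; Swipes drive controller yaw and pitch with an interpolated fade-out, while a delay-closed gate and distance threshold detect single taps.
; Taps trace from the screen, then straight down for the SimpleMoveToLocation goal, spawning a move indicator and notifying the HUD.
; Timelines turn the view toward the goal or move direction and optionally level pitch afterward.
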(event EventTick
  (params (DeltaSeconds :type Float%20%28single-precision%29))
  ;[1 1 1] Init
  (CallFunction|TouchTick DeltaSeconds))

(event EventBeginPlay
  ;[1 1 1] Init
  (Variables|Refs|SetPlayerController (Game|GetPlayerController 0))
  (bind _asbp_mobile_navigation_hud (Utilities|Casting|CastToBP_MobileNavigation_HUD (HUD|GetHUD (Variables|Refs|GetPlayerController))))
  (Variables|Refs|SetHUD _asbp_mobile_navigation_hud))

(event Custom|Touch%20Tick
  (params (DeltaTIme :type Float%20%28single-precision%29))
  ;[1 1 1] Swipe to Look
  (Variables|TouchInputLocalVars|SetInterpVal (CallFunction|Vector2DInterp (Variables|TouchInputLocalVars|GetInterpVal) "(X=0.000000,Y=0.000000)" (Variables|TouchInputLocalVars|GetInterpSpeed) DeltaTIme))
  (Utilities|TouchInput-SetControllerYawandPitch (Variables|TouchInputLocalVars|GetInterpVal)))

(event Custom|Single%20Tap
  (params (non%20Relative%20Location :type Vector%202D%20Structure))
  (bind _playercontroller (Variables|Refs|GetPlayerController))
  (bind (_worldlocation _worlddirection) (Class|PlayerController|DeprojectScreenPositiontoWorld _playercontroller (.x non%20Relative%20Location) (.y non%20Relative%20Location)))
  (bind _result (CallFunction|OffsetinDirection _worldlocation _worlddirection 2e+03))
  ;[1 1 1] Tap To Move - Movement
  (bind (_outhit _returnvalue) (Collision|LineTraceByChannel _worldlocation _result "TraceTypeQuery1" false 0 "None")) ; The first trace goes in the desired direction
  (if _returnvalue
    (if (not (CallFunction|TouchInput-TooClose (CallFunction|DistanceBetween (Transformation|GetActorLocation) (.Location (Collision|BreakHitResult _outhit)))))
      (Utilities|TouchInput-TaptoMoveAction (CallFunction|OffsetinDirection (.Location (Collision|BreakHitResult _outhit)) (.Normal (Collision|BreakHitResult _outhit)) (Variables|/Script/Engine.CapsuleComponent|GetCapsuleRadius (Variables|Collision|GetCapsuleComponent))) ; If we hit something, it is offset by capsule radius along hitnormal
        (:Out
          (Default|TaptoMoveStart (Variables|Refs|GetHUD) (.x non%20Relative%20Location) (.y non%20Relative%20Location) :!label _label) ; We only show hud stuff when the move definitely happens
        )))
    (else
      (Utilities|TouchInput-TaptoMoveAction _result ; Starts where first trace ends if nothing is hit
        (:Out
          (goto _label))))))

(event Custom|Stop%20Look%20At%20Tap%20To%20Move
  (bind _returnvalue (Transformation|GetActorLocation))
  (bind _returnvalue_2 (Pawn|GetControlRotation :!class /Script/Engine.Pawn))
  (bind (_roll _pitch _yaw) (Math|Rotator|BreakRotator _returnvalue_2))
  ;[1 1 1] Tap to Move - Look at Location
  (Utilities|FlowControl|Sequence
    (:then_0
      (bind _interpspeed (Timeline|Look%20At%20Tap%20To%20Move Stop) ; Adjust how fast we look at movement goal
        (:Update
          (if (CallFunction|TouchInput-TooClose (CallFunction|DistanceBetween _returnvalue (stale Custom|Look%20At%20Tap%20To%20Move%20Loc Location)))
            (Variables|TouchInputLocalVars|SetAutoResetViewrot true)
            (CallFunction|TriggerAutoResetViewrot)
            (else
              (Utilities|TouchInput-InterpLookatRotation (Math|Rotator|FindLookatRotation _returnvalue (CallFunction|TouchInput-GetLookatLocation (stale Custom|Look%20At%20Tap%20To%20Move%20Loc Location))) _interpspeed) ; Interpolate the view rotation to the movement goal
            )))))
    (:then_1
      (Utilities|TouchInput-CheckAutoResetViewrot
        (:%20%20%20%20
          (bind _interpspeed_2 (Timeline|Reset%20Look%20At%20Rotation Stop) ; Adjust how fast viewrotation is reset
            (:Update
              (Utilities|TouchInput-InterpLookatRotation (Math|Rotator|MakeRotator _roll 0.0 _yaw) _interpspeed_2) ; Reset the view rotation once we stop
            )))))))

(event Custom|Tap%20End
  (params (Location :type Vector%202D%20Structure) (Non%20Relative%20Location :type Vector%202D%20Structure))
  ;[1 1 1] Tap to Move - Check for single tap based on time and swipe lenght
  (Utilities|FlowControl|Gate true
    (:Exit
      (if (< (* (CallFunction|DistanceBetween(Vector2D) Location (Variables|TouchInputLocalVars|GetTapStart)) 1e+02) (Variables|TouchInput|GetSIngleTapSwipeThreshold)) ; Check if tap or swipe
        (CallFunction|SingleTap Non%20Relative%20Location)))))

(event Custom|Touch%20Moved
  (params (Location :type Vector%202D%20Structure))
  ;[1 1 1] Swipe to Look
  (Variables|TouchInputLocalVars|SetInterpVal (CallFunction|Vector2D*Vector2D (- Location (Variables|TouchInputLocalVars|GetTouchStart)) (Variables|TouchInput|GetSwipeYawAndPitchScale)))
  (Utilities|TouchInput-SetControllerYawandPitch (Variables|TouchInputLocalVars|GetInterpVal)
    (:out
      (Variables|TouchInputLocalVars|SetTouchStart Location) ; Clear this each tick to make it work like axis input value
    )))

(event Custom|Touch%20Began
  (params (Location :type Vector%202D%20Structure))
  ;[1 1 1] Swipe to Look
  (Variables|TouchInputLocalVars|SetTouchStart Location)
  (Variables|TouchInputLocalVars|SetInterpSpeed 1.0) ; Speed when touching, set to 1 so it is pretty much ignored and only the direct input is used
)

(event Custom|Trigger%20Auto%20Reset%20Viewrot
  (bind _returnvalue (Transformation|GetActorLocation))
  (bind _returnvalue_2 (Pawn|GetControlRotation :!class /Script/Engine.Pawn))
  (bind (_roll _pitch _yaw) (Math|Rotator|BreakRotator _returnvalue_2))
  ;[1 1 1] Tap to Move - Look at Location
  (Utilities|FlowControl|Sequence
    (:then_0
      (bind _interpspeed (Timeline|Look%20At%20Tap%20To%20Move Stop) ; Adjust how fast we look at movement goal
        (:Update
          (if (CallFunction|TouchInput-TooClose (CallFunction|DistanceBetween _returnvalue (stale Custom|Look%20At%20Tap%20To%20Move%20Loc Location)))
            (Variables|TouchInputLocalVars|SetAutoResetViewrot true)
            (CallFunction|TriggerAutoResetViewrot)
            (else
              (Utilities|TouchInput-InterpLookatRotation (Math|Rotator|FindLookatRotation _returnvalue (CallFunction|TouchInput-GetLookatLocation (stale Custom|Look%20At%20Tap%20To%20Move%20Loc Location))) _interpspeed) ; Interpolate the view rotation to the movement goal
            )))))
    (:then_1
      (if (and (Variables|TouchInput|GetAuto%20Reset%20View%20Rotation) (Variables|TouchInputLocalVars|GetAutoResetViewrot)) ; Only play if desired
        (bind _interpspeed_2 (Timeline|Reset%20Look%20At%20Rotation PlayFromStart) ; Adjust how fast viewrotation is reset
          (:Update
            (Utilities|TouchInput-InterpLookatRotation (Math|Rotator|MakeRotator _roll 0.0 _yaw) _interpspeed_2) ; Reset the view rotation once we stop
          ))))))

(event Custom|Look%20At%20Tap%20To%20Move%20Loc
  (params (Location :type Vector))
  (bind _returnvalue (Transformation|GetActorLocation))
  ;[1 1 1] Tap to Move - Look at Location
  (bind _interpspeed (Timeline|Look%20At%20Tap%20To%20Move PlayFromStart) ; Adjust how fast we look at movement goal
    (:Update
      (if (CallFunction|TouchInput-TooClose (CallFunction|DistanceBetween _returnvalue Location))
        (Variables|TouchInputLocalVars|SetAutoResetViewrot true)
        (CallFunction|TriggerAutoResetViewrot)
        (else
          (Utilities|TouchInput-InterpLookatRotation (Math|Rotator|FindLookatRotation _returnvalue (CallFunction|TouchInput-GetLookatLocation Location)) _interpspeed) ; Interpolate the view rotation to the movement goal
        )))))

(event Custom|Touch%20Ended
  (params (Location :type Vector%202D%20Structure))
  ;[1 1 1] Swipe to Look
  (Variables|TouchInputLocalVars|SetInterpSpeed (Variables|TouchInput|GetSwipeFadeInterpSpeed)) ; Speed when fading out
)

(event Custom|Tap%20Start
  (params (Location :type Vector%202D%20Structure))
  ;[1 1 1] Tap to Move - Check for single tap based on time and swipe lenght
  (Utilities|FlowControl|Sequence
    (:then_0
      (Variables|TouchInputLocalVars|SetTapStart Location)
      (CallFunction|StopLookatTaptoMove)
      (Utilities|FlowControl|Delay (Variables|TouchInput|GetSingleTapDelay)) ; Check time threshold and close gate if passed
      (Utilities|FlowControl|Gate true) ; enters at Close
    )
    (:then_1
      (Utilities|FlowControl|Gate true) ; enters at Open
    )))

(fn ConstructionScript)

(fn TouchInput-GetLookatLocation
  (params (Look%20At :type Vector))
  (bind _returnvalue (Transformation|GetVelocity))
  (bind _looklocationoffset (Variables|TouchInput|GetLookLocationOffset))
  (bind _returnvalue_2 (Math|Vector|MakeVector 0.0 0.0 _looklocationoffset))
  (bind _returnvalue_3 (+ Look%20At _returnvalue_2))
  (bind _returnvalue_4 (+ _returnvalue _returnvalue_3))
  (bind (_x _y) (Math|Vector|BreakVector _returnvalue_4))
  ;[1 1 1] Use Velocity to get actual move dir
  (return (Math|Vector|SelectVector (Math|Vector|MakeVector _x _y (.Z (Math|Vector|BreakVector _returnvalue_3))) _returnvalue_3 (and (Variables|TouchInput|GetLookInMoveDirection) (> (Math|Vector|VectorLength _returnvalue) 0.0)))))

(fn TouchInput-TooClose
  (params (A :type Float%20%28single-precision%29))
  (return (< A (Variables|TouchInput|GetMinTapToMoveDist))))