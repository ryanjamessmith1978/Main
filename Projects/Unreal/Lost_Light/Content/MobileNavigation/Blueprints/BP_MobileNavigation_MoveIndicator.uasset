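; Move indicator actor for mobile navigation that animates in when spawned and removes itself when the navigation pawn reaches it.
; On BeginPlay a timeline drives the actor's uniform scale through the ScaleUp curve.
; The first actor overlap passes a DoOnce, then a class check for BP_MobileNavigation_Pawn starts the ScaleDown timeline, which destroys the actor when finished.
; DoOnce precedes the class check, so any first overlapping actor consumes it.
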(event EventActorBeginOverlap
  (params (OtherActor :type Actor%20Object%20Reference))
  (Utilities|FlowControl|DoOnce false
    (:Completed
      (if (CallFunction|IsClassOf OtherActor "/Game/MobileNavigation/Blueprints/BP_MobileNavigation_Pawn.BP_MobileNavigation_Pawn_C")
        (bind _scale (Timeline|ScaleDown PlayFromStart)
          (:Update
            (Transformation|SetActorScale3D (Math|Conversions|ToVector(Float) _scale)))
          (:Finished
            (Actor|DestroyActor)))))))

(event EventBeginPlay
  (bind _scale (Timeline|ScaleUp PlayFromStart)
    (:Update
      (Transformation|SetActorScale3D (Math|Conversions|ToVector(Float) _scale)))))

(fn ConstructionScript)