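; Player controller for mobile navigation that captures touch input and forwards it to BP_MobileNavigation_Pawn, cached on BeginPlay.
; Press and release start and end both touch and tap on the pawn, while Tick polls the finger state to send movement.
; Moved locations are scaled by screen size for consistency across devices.
; Touches are handled on the pawn because yaw/pitch input only works from there.
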(event Custom|InputTouch%20Tick
  ;[1 1 1] Send Touch Input to Pawn
  (if (.bIsCurrentlyPressed (Class|PlayerController|GetInputTouchState (stale Input|TouchEvents|InputTouch FingerIndex)))
    (Utilities|TouchInput-FireEvents (CallFunction|ScalebyScreenSize (Math|Vector2D|MakeVector2D (.LocationX (Class|PlayerController|GetInputTouchState (stale Input|TouchEvents|InputTouch FingerIndex))) (.LocationY (Class|PlayerController|GetInputTouchState (stale Input|TouchEvents|InputTouch FingerIndex))))) (Math|Vector2D|MakeVector2D (.LocationX (Class|PlayerController|GetInputTouchState (stale Input|TouchEvents|InputTouch FingerIndex))) (.LocationY (Class|PlayerController|GetInputTouchState (stale Input|TouchEvents|InputTouch FingerIndex))))) ; enters at Moved
  ))

(event EventTick
  (params (DeltaSeconds :type Float%20%28single-precision%29))
  ;[1 1 1] Init
  (CallFunction|InputTouchTick))

(event EventBeginPlay
  ;[1 1 1] Init
  (bind _asbp_mobile_navigation_pawn (Utilities|Casting|CastToBP_MobileNavigation_Pawn (Game|Player|GetPlayerPawn 0)))
  (Variables|Refs|SetMyPawn _asbp_mobile_navigation_pawn))

(event Input|TouchEvents|InputTouch
  (params (Location :type Vector) (FingerIndex :type ETouchIndex%20Enum :default "Touch1"))
  (bind (_locationx _locationy _biscurrentlypressed) (Class|PlayerController|GetInputTouchState FingerIndex))
  (bind _returnvalue (Math|Vector2D|MakeVector2D _locationx _locationy))
  ;[1 1 1] Send Touch Input to Pawn
  (:Pressed
    (Utilities|TouchInput-FireEvents (CallFunction|ScalebyScreenSize _returnvalue) _returnvalue :!label _label) ; We send it to the character, because the yaw/pitch input only work from there
  )
  (:Released
    (goto _label End)))

(fn ConstructionScript)