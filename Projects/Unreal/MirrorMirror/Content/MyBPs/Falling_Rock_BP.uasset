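; Falling rock hazard that damages the player on contact and shatters through a destructible component.
; Hits on an MMCharacter subtract a small random amount from PlayerHealth stored directly on MyHUD, with a brief delay flag preventing rapid repeat damage.
; On fracture it plays a crash sound at the hit point, activates a radial force and destroys itself a few seconds later.
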(event OnComponentHit(DestructibleComponent)
  (params (OtherActor :type Actor%20Object%20Reference) (OtherComp :type Primitive%20Component%20Object%20Reference) (NormalImpulse :type Vector) (Hit :type Hit%20Result%20Structure%20%28by%20ref%29))
  (bind _myhud (Variables|Default|GetMyHUD))
  (Utilities|Casting|CastToMMCharacter OtherActor)
  (if (not (Variables|Default|GetplayerTakingDamage))
    (Variables|/Game/MyBPs/MyHUD/MyHUD.MyHUD_C|SetPlayerHealth _myhud (- (Variables|/Game/MyBPs/MyHUD/MyHUD.MyHUD_C|GetPlayerHealth _myhud) (Math|Random|RandomFloatinRange 0.1 0.2)))
    (Variables|Default|SetplayerTakingDamage true)
    (Utilities|FlowControl|Delay 0.3)
    (Variables|Default|SetplayerTakingDamage false)))

(event OnComponentFracture(DestructibleComponent)
  (params (HitPoint :type Vector%20%28by%20ref%29) (HitDirection :type Vector%20%28by%20ref%29 :default "0, 0, 0"))
  (Audio|SpawnSoundatLocation "/Game/MyBPs/RockCrash_3.RockCrash_3" HitPoint "0, 0, 0" 0.75)
  (Components|Activation|Activate (Variables|Default|GetRadialForce) false)
  (Utilities|FlowControl|Delay 3.0)
  (Actor|DestroyActor))

(event EventBeginPlay
  (bind _asmy_hud (Utilities|Casting|CastToMyHUD (HUD|GetHUD (Game|GetPlayerController 0))))
  (Variables|Default|SetMyHUD _asmy_hud))

(fn ConstructionScript)