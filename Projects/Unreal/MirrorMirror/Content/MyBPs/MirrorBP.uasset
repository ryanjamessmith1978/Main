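; Puzzle mirror actor that bounces a light beam toward an exit switch and can be turned by the player.
; Clicking it while the pawn overlaps its box rotates it 45 degrees with a stone-scrape sound after a short delay.
; ReflectLight traces along the incoming hit normal, sizes and shows the beam, then recursively calls the next mirror hit or triggers the ExitSwitch to open the door.
; A timeline-based rotation remains unwired.
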(event Custom|BounceLight
  ;[1 1 1] Bounce Light
)

(event EventTick
  (params (DeltaSeconds :type Float%20%28single-precision%29))
  (bind _returnvalue (Game|GetPlayerController 0))
  (bind _box (Variables|Default|GetBox))
  (bind _returnvalue_2 (Pawn|GetControlledPawn _returnvalue))
  (bind _returnvalue_3 (Collision|IsOverlappingActor _box _returnvalue_2 :!class /Script/Engine.PrimitiveComponent))
  ;[1 1 1] Rotate Mirror with Click Player 1 (index 0)
  (if (not (Variables|Default|GetReflecting))
    (Rendering|SetVisibility (Variables|Default|GetLightBeamTexture) false false))
  (if _returnvalue_3
    (Variables|Default|SetOverlapMirror _returnvalue_3)
    (if (Variables|Default|GetOverlapMirror)
      (Input|EnableInput _returnvalue_2 0)
      (else
        (Input|DisableInput _returnvalue_2 0)))))

(event EventBeginPlay
  ;[1 1 1] Play timed functions Bounce Light and Click Mirror on Loop at Start
  (bind _asmy_game_mode (Utilities|Casting|CastToMyGameMode (Game|GetGameMode)))
  (Variables|Default|SetGameModeRef _asmy_game_mode))

(event MouseInput|EventActorOnClicked
  ;[1 1 1] Rotate Mirror with Click Player 1 (index 0)
  (if (Variables|Default|GetOverlapMirror)
    (Utilities|FlowControl|Delay 0.4)
    (CallFunction|RotateMirror)))

(fn ConstructionScript
  (Variables|Default|SetRotation (Transformation|GetActorRotation)))

(fn ReflectLight
  (params (HitLocation :type Vector) (HitNormal :type Vector))
  (bind _mirrorbeam (Variables|Default|GetMirrorBeam))
  (Variables|Default|SetReflecting true)
  (bind _output_get (Variables|Default|SetStarting%20Vector HitLocation))
  (bind _outhit (Collision|LineTraceByChannel _output_get (+ HitLocation (* HitNormal 7.5e+03)) "TraceTypeQuery1" false 0 "None"))
  (bind _output_get_2 (Variables|Default|SetBeamDistance (Math|Vector|VectorLength (- (Variables|Default|GetStarting%20Vector) (.ImpactPoint (Collision|BreakHitResult _outhit))))))
  (Rendering|Lighting|SetAttenuationRadius _mirrorbeam _output_get_2)
  (Rendering|SetVisibility _mirrorbeam true false)
  (Rendering|SetVisibility (Variables|Default|GetLightBeamTexture) true false)
  (bind _asexit_switch (Utilities|Casting|CastToExitSwitch (.HitActor (Collision|BreakHitResult _outhit)))
    (:then
      ;[1 1 1] Open door
      (Default|SwitchinWall _asexit_switch)
      (Default|OpenSesame _asexit_switch))
    (:CastFailed
      (bind _asmirror_bp (Utilities|Casting|CastToMirrorBP (.HitActor (Collision|BreakHitResult _outhit))))
      (CallFunction|ReflectLight _asmirror_bp (.ImpactPoint (Collision|BreakHitResult _outhit)) (.ImpactNormal (Collision|BreakHitResult _outhit))))))

(fn RotateMirror
  (bind _defaultsceneroot (Variables|Default|GetDefaultSceneRoot))
  (Transformation|SetWorldRotation _defaultsceneroot (Math|Rotator|MakeRotator (.Roll (Math|Rotator|BreakRotator (Variables|Default|GetRotation))) (.Pitch (Math|Rotator|BreakRotator (Variables|Default|GetRotation))) (+ (.Yaw (Math|Rotator|BreakRotator (Variables|Default|GetRotation))) 45.0)) false false)
  (Variables|Default|SetRotation (Math|Rotator|MakeRotator (.Roll (Math|Rotator|BreakRotator (Variables|Default|GetRotation))) (.Pitch (Math|Rotator|BreakRotator (Variables|Default|GetRotation))) (+ (.Yaw (Math|Rotator|BreakRotator (Variables|Default|GetRotation))) 45.0)))
  (Audio|PlaySoundatLocation "/Game/MyBPs/heavy_stone_slab_scrape_or_drag_co_1.heavy_stone_slab_scrape_or_drag_co_1" (Transformation|GetWorldLocation _defaultsceneroot)))