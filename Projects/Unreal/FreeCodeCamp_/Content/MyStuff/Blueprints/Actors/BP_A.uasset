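; BP_A is an Actor Blueprint that appears to be a networking test for replicated floats and RPCs.
; OnRep_RandomFloat prints RandomFloat, while the SetSomeFloatRPC event randomizes AnotherRandomFloat and prints it for five seconds.
; BeginPlay's server check and the SetSomeFloat_MC event do nothing.
; The server-only RandomFloat assignment and both RPC calls are disconnected, so nothing in this graph triggers them.
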(event Custom|SetSomeFloatRPC
  (bind _output_get (Variables|Default|SetAnotherRandomFloat (Math|Random|RandomFloat)))
  (Development|PrintString (Utilities|String|ToString(Float) _output_get) true true "(R=0.000000,G=0.660000,B=1.000000,A=1.000000)" 5.0))

(event Custom|SetSomeFloat_MC)

(event EventBeginPlay
  (if (Networking|IsServer)
    _))

(fn ConstructionScript)

(fn OnRepRandomFloat
  (Development|PrintString (Utilities|String|ToString(Float) (Variables|Default|GetRandomFloat))))