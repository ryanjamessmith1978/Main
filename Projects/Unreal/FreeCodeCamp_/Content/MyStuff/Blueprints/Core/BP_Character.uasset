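; Player character that serves as a test bed for RPCs, damage and pickup removal, alongside movement, look and crouch input.
; On the server, BeginPlay spawns an owned BP_DamageActor, whose server, client and multicast RPCs are triggered by debug keys.
; Right click applies random point damage via camera line trace; Interact destroys overlapping pickups and Shoot calls RemovePickup in C++.
; The timer setup for GetReferences, which fetches look sensitivity from the controller, is disconnected.
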(event Custom|Local_RPC_Call
  ;[0.15 0.15 0.15 0.5] Local RPC Call
  (Development|PrintString "RPC Server Call from Character"))

(event EventTestBPFunc
  (params (x :type Integer))
  ;[0.15 0.15 0.15 0.5] C++ Interface Examples with PrintString
)

(event EventBeginPlay
  ;[0.15 0.15 0.15 0.5] Begin Play
  (Utilities|Casting|CastToBP_MyGameMode (Game|GetGameMode)
    (:then
      _)
    (:CastFailed
      _))
  (if (Networking|IsServer)
    ;;[0.15 0.15 0.15 0.5] Spawn needs to be on server
    (bind _returnvalue (Game|SpawnActorfromClass "/Game/MyStuff/Blueprints/Actors/BP_DamageActor.BP_DamageActor_C" (Math|Transform|MakeTransform (Variables|Default|GetSpawn%20Transform%20Location) "0, 0, 0" "1.000000,1.000000,1.000000") "Undefined" "MultiplyWithRoot" self 0.0 0))
    (Variables|Default|SetDamageActor_OBJ _returnvalue)))

(event EventTick
  (params (DeltaSeconds :type Float%20%28single-precision%29))
  ;[0.15 0.15 0.15 0.5] Event Tick
)

(event EventTestBPImp
  (params (x :type Float%20%28single-precision%29))
  ;[0.15 0.15 0.15 0.5] C++ Interface Examples with PrintString
)

(event EventOnEndCrouch
  (params (HalfHeightAdjust :type Float%20%28single-precision%29) (ScaledHalfHeightAdjust :type Float%20%28single-precision%29))
  (Development|PrintString "DONE CROUCHING"))

(event Input|ActionEvents|InputActionInteract
  (params (Key :type Key%20Structure :default "None"))
  ;[0.15 0.15 0.15 0.5] Interact and Destroy
  (:Pressed
    (for _array_element (Collision|GetOverlappingActors (Variables|Default|GetCapsuleComponent) "/Game/MyStuff/Blueprints/Actors/BP_MyPickup.BP_MyPickup_C" :!class /Script/Engine.PrimitiveComponent) :!label _label
      (if (Utilities|IsValid _array_element)
        (Actor|DestroyActor _array_element)
        (goto _label)))))

(event Input|ActionEvents|InputActionShoot
  (params (Key :type Key%20Structure :default "None"))
  ;[0.15 0.15 0.15 0.5] Shoot Pickup - Calls CPP function - and Destroys it
  (:Pressed
    (Class|CPPCharacter|RemovePickup)))

(event Input|AxisEvents|InputAxisMoveForward
  (params (AxisValue :type Float%20%28single-precision%29))
  ;[0.15 0.15 0.15 0.5] Movement
  (Pawn|Input|AddMovementInput (Transformation|GetActorForwardVector) AxisValue false))

(event Input|AxisEvents|InputAxisMoveUp
  (params (AxisValue :type Float%20%28single-precision%29))
  (Pawn|Input|AddMovementInput (Transformation|GetActorUpVector) AxisValue false))

(event Input|AxisEvents|InputAxisMoveSide
  (params (AxisValue :type Float%20%28single-precision%29))
  ;[0.15 0.15 0.15 0.5] Movement
  (Pawn|Input|AddMovementInput (Transformation|GetActorRightVector) AxisValue false))

(event Input|AxisEvents|InputAxisLookAround
  (params (AxisValue :type Float%20%28single-precision%29))
  ;[0.15 0.15 0.15 0.5] Look
  (Pawn|Input|AddControllerYawInput (* AxisValue (Variables|Default|GetLocal%20Sensitivity))))

(event Input|AxisEvents|InputAxisLookUp
  (params (AxisValue :type Float%20%28single-precision%29))
  ;[0.15 0.15 0.15 0.5] Look
  (Pawn|Input|AddControllerPitchInput (* AxisValue (Variables|Default|GetLocal%20Sensitivity))))

(event Input|MouseEvents|RightMouseButton
  (params (Key :type Key%20Structure :default "None"))
  ;[0.15 0.15 0.15 0.5] Point Damage
  (:Pressed
    (CallFunction|PointDamage)))

(event Input|KeyboardEvents|C
  (params (Key :type Key%20Structure :default "None"))
  (:Pressed
    (Character|Crouch))
  (:Released
    (Character|UnCrouch self)))

(event Input|KeyboardEvents|M
  (params (Key :type Key%20Structure :default "None"))
  (bind _damageactor_obj (Variables|Default|GetDamageActor_OBJ))
  ;[0.15 0.15 0.15 0.5] MultiCast Call - ServerSide (On Damaged Actor)
  (:Pressed
    (if (Utilities|IsValid _damageactor_obj)
      (Default|ServerRPCCall _damageactor_obj true))))

(event Input|KeyboardEvents|R
  (params (Key :type Key%20Structure :default "None"))
  (bind _damageactor_obj (Variables|Default|GetDamageActor_OBJ))
  ;[0.15 0.15 0.15 0.5] Remote Procedural Call - Server Side (on Damaged Actor)
  (:Pressed
    (if (Utilities|IsValid _damageactor_obj)
      ;;[0.15 0.15 0.15 0.5] If this Custom Event is set to run on the Client in the Damaged Actor class, but the spawned actor does not have a reference to the owning Character, then the Client Call will not be displayed, only the server call
      (Default|ServerRPCCall _damageactor_obj false))))

(event Input|KeyboardEvents|L
  (params (Key :type Key%20Structure :default "None"))
  ;[0.15 0.15 0.15 0.5] Local RPC Call
  (:Pressed
    (CallFunction|LocalRPCCall)))

(event Input|KeyboardEvents|F
  (params (Key :type Key%20Structure :default "None"))
  (bind _damageactor_obj (Variables|Default|GetDamageActor_OBJ))
  ;[0.15 0.15 0.15 0.5] RPC - Client Side (On Damaged Actor)
  (:Pressed
    (if (Utilities|IsValid _damageactor_obj)
      (Default|ClientRPC _damageactor_obj))))

(fn ConstructionScript)

(fn GetReferences
  (bind _asbp_player_controller (Utilities|Casting|CastToBP_PlayerController (Game|GetPlayerController 0)))
  (bind _output_get (Variables|Default|SetAs%20BP%20Player%20Controller _asbp_player_controller))
  (Variables|Default|SetLocal%20Sensitivity (Default|GetSensitivity _output_get))
  ;[0.15 0.15 0.15 0.5] Stop Timer external from Call Timer Function
  (Utilities|Time|ClearandInvalidateTimerbyHandle (Variables|Default|GetInitTimer)))

(fn PointDamage
  (bind _returnvalue (Game|GetPlayerCameraManager 0))
  (bind _returnvalue_2 (Transformation|GetActorLocation _returnvalue))
  (bind _outhit (Collision|LineTraceByChannel _returnvalue_2 (+ _returnvalue_2 (* (Transformation|GetActorForwardVector _returnvalue) 2.5e+04)) "TraceTypeQuery1" false 0 "Persistent"))
  (Game|Damage|ApplyPointDamage (.HitActor (Collision|BreakHitResult _outhit)) (Math|Random|RandomFloatinRange 2e+01 5e+01) (Math|Vector|GetUnitDirection(Vector) (.TraceStart (Collision|BreakHitResult _outhit)) (.Location (Collision|BreakHitResult _outhit))) _outhit 0 self))