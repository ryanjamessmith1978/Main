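; Actor component that owns health, healing, damage and death for its actor.
; TakeDamage routes through the CanBeDamaged macro to block, damage or ignore hits, then fires blocked, death, or, for interrupting hits, damage-type and response dispatchers.
; Heal clamps Health to MaxHealth while alive.
; TakeDamage feeds the component's own IsInvincible and IsBlocking into the macro's override inputs, so invincibility never prevents damage and DamageInfo cannot bypass blocking.
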(event EventBeginPlay)

(event EventTick
  (params (DeltaSeconds :type Float%20%28single-precision%29)))

(fn Heal
  (params (HealAmount :type Float%20%28double-precision%29))
  (if (not (Variables|Default|GetbIsDead))
    (bind _output_get (Variables|Default|SetHealth (Math|Float|Clamp(Float) (+ HealAmount (Variables|Default|GetHealth)) 0.0 (Variables|Default|GetMaxHealth))))
    (return _output_get)))

(fn TakeDamage
  (params (DamageInfo :type Damage%20Info%20Structure))
  (bind (_amountofdamage _damagetype _damageresponse _bisdamageinvincible _bisblockable _bisparryable _bisanimationinterrupt) (Utilities|Struct|BreakDamageInfo DamageInfo))
  (Utilities|CanbeDamaged (Variables|Default|GetbIsInvincible) (Variables|Default|GetbIsBlocking)
    (:BlockDamage
      (Default|CallOnBlocked _bisparryable)
      (return false))
    (:DoDamage
      (bind _output_get (Variables|Default|SetHealth (- (Variables|Default|GetHealth) _amountofdamage)))
      (Development|PrintString (Utilities|String|ToString(Float) _output_get))
      (if (<= (Variables|Default|GetHealth) 0.0)
        (Variables|Default|SetbIsDead true)
        (Default|CallOnDeath)
        (return true)
        (elif (or (Variables|Default|GetbIsInterruptable) _bisanimationinterrupt)
          (Default|CallOnDamageType _damagetype)
          (Default|CallOnDamageResponse _damageresponse)
          (return true))))
    (:NoDamage
      (return false))))