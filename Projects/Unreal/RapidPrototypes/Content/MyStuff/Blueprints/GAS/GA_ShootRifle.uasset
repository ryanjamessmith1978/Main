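; Gameplay Ability that fires the first-person character's rifle, launching a fireball projectile and ending immediately.
; It spawns the projectile at the mesh's "Ammo" socket plus a camera-rotated offset, aimed along player 0's camera.
; It plays a firing sound there, attaches an explosion emitter to the projectile, and plays the shoot montage on player 0's first-person mesh.
; The ability never calls CommitAbility.
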(event Ability|EventActivateAbility
  (bind _returnvalue (Game|GetPlayerCameraManager 0))
  (bind _returnvalue_2 (Camera|GetCameraRotation _returnvalue))
  ;[0.05 0.05 0.05] Projectile Spawn Logic
  (bind _asbp_first_person_character_gas (Utilities|Casting|CastToBP_FirstPersonCharacterGAS (Ability|GetAvatarActorfromActorInfo)))
  (Variables|Default|SetAs%20BP%20First%20Person%20Character%20GAS _asbp_first_person_character_gas)
  (bind _returnvalue_3 (Game|SpawnActorfromClass "/Game/MyStuff/Blueprints/DamageSystem/DamageTypes_StatusFX/BP_FPSProjectile_FireBall.BP_FPSProjectile_FireBall_C" (Math|Transform|MakeTransform (+ (Transformation|GetSocketLocation (Variables|/Script/Engine.Character|GetMesh (Variables|Default|GetAs%20BP%20First%20Person%20Character%20GAS)) "Ammo") (Math|Vector|RotateVector (Variables|Default|GetProjectileOffset) _returnvalue_2)) _returnvalue_2) "Undefined" "OverrideRootScale" 0 0))
  (Audio|PlaySoundatLocation "/Game/MyStuff/Assets/FPWeapon/Audio/FirstPersonTemplateWeaponFire02.FirstPersonTemplateWeaponFire02" (+ (Transformation|GetSocketLocation (Variables|/Script/Engine.Character|GetMesh (Variables|Default|GetAs%20BP%20First%20Person%20Character%20GAS)) "Ammo") (Math|Vector|RotateVector (Variables|Default|GetProjectileOffset) _returnvalue_2)) "0, 0, 0" 1.0 1.0 0.0 0 0 0 0) ; Play firing sound
  (Effects|SpawnEmitterAttached "/Game/StarterContent/Particles/P_Explosion.P_Explosion" (Variables|/Game/MyStuff/Blueprints/DamageSystem/DamageTypes_StatusFX/BP_FPSProjectile_FireBall.BP_FPSProjectile_FireBall_C|GetSphere _returnvalue_3) "None" "0, 0, 0" "0, 0, 0" "1.000000,1.000000,1.000000" "SnapToTarget")
  (bind _asbp_first_person_character_gas_2 (Utilities|Casting|CastToBP_FirstPersonCharacterGAS (Game|GetPlayerCharacter 0)))
  (Animation|Montage|MontagePlay (Components|SkeletalMesh|GetAnimInstance (Variables|/Game/MyStuff/Blueprints/GAS/BP_FirstPersonCharacterGAS.BP_FirstPersonCharacterGAS_C|GetFirstPersonMesh _asbp_first_person_character_gas_2)) "/Game/Characters/FirstPersonArms/Animations/FP_Rifle_Shoot_Montage.FP_Rifle_Shoot_Montage" 1.0 "MontageLength" 0.0 true)
  (Ability|EndAbility))