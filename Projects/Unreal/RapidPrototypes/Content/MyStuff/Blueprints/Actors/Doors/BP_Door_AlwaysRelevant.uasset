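; BP_Door_AlwaysRelevant is an interactable door for a replication setup, named for always-relevant networking.
; InteractDoor calls the MC (apparently multicast) open event, which plays a timeline that lerps the door's world rotation from start to end.
; When a BP_ReplicationTPPChar leaves the overlap trigger, the MC close event reverses that same timeline from the end.
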(event OnComponentEndOverlap(OverlapTrigger)
  (params (OverlappedComponent :type Primitive%20Component%20Object%20Reference) (OtherActor :type Actor%20Object%20Reference) (OtherComp :type Primitive%20Component%20Object%20Reference) (OtherBodyIndex :type Integer))
  (Utilities|Casting|CastToBP_ReplicationTPPChar OtherActor)
  (CallFunction|MCCloseDoor))

(event Custom|MC_OpenDoor
  (bind _doortrack (Timeline|OpenDoor_TL PlayFromStart)
    (:Update
      (Transformation|SetWorldRotation (Variables|Default|GetDoor) (Math|Rotator|Lerp(Rotator) (Variables|Default|GetStartingRot) (Variables|Default|GetEndingRot) _doortrack) false false))))

(event Custom|MC_CloseDoor
  (bind _doortrack (Timeline|OpenDoor_TL ReverseFromEnd)
    (:Update
      (Transformation|SetWorldRotation (Variables|Default|GetDoor) (Math|Rotator|Lerp(Rotator) (Variables|Default|GetStartingRot) (Variables|Default|GetEndingRot) _doortrack) false false))))

(event EventInteractDoor
  (CallFunction|MCOpenDoor))

(event EventBeginPlay
  (|CallParentFunction))

(fn ConstructionScript
  (|CallParentFunction))