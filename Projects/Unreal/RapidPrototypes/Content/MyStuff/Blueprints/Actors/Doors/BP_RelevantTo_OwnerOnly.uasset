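; BP_RelevantTo_OwnerOnly is an interactable door, apparently a replication example for owner-only relevancy.
; InteractDoor fires paired SR and OC open events, named for server and owning-client execution, which play one timeline that lerps the door's world rotation.
; When a BP_ReplicationTPPChar that owns the door leaves the trigger, paired close events reverse that timeline from the end.
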(event OnComponentEndOverlap(OverlapTrigger)
  (params (OverlappedComponent :type Primitive%20Component%20Object%20Reference) (OtherActor :type Actor%20Object%20Reference) (OtherComp :type Primitive%20Component%20Object%20Reference) (OtherBodyIndex :type Integer))
  (bind _asbp_replication_tppchar (Utilities|Casting|CastToBP_ReplicationTPPChar OtherActor))
  (if (== (Components|GetOwner) _asbp_replication_tppchar)
    (CallFunction|SRCloseDoor)
    (CallFunction|OCCloseDoor)))

(event Custom|OC_OpenDoor
  (bind _doortrack (Timeline|Timeline PlayFromStart)
    (:Update
      (Transformation|SetWorldRotation (Variables|Default|GetDoor) (Math|Rotator|Lerp(Rotator) (Variables|Default|GetStartingRot) (Variables|Default|GetEndingRot) _doortrack) false false))))

(event Custom|SR_OpenDoor
  (bind _doortrack (Timeline|Timeline PlayFromStart)
    (:Update
      (Transformation|SetWorldRotation (Variables|Default|GetDoor) (Math|Rotator|Lerp(Rotator) (Variables|Default|GetStartingRot) (Variables|Default|GetEndingRot) _doortrack) false false))))

(event Custom|OC_CloseDoor
  (bind _doortrack (Timeline|Timeline ReverseFromEnd)
    (:Update
      (Transformation|SetWorldRotation (Variables|Default|GetDoor) (Math|Rotator|Lerp(Rotator) (Variables|Default|GetStartingRot) (Variables|Default|GetEndingRot) _doortrack) false false))))

(event Custom|SR_CloseDoor
  (bind _doortrack (Timeline|Timeline ReverseFromEnd)
    (:Update
      (Transformation|SetWorldRotation (Variables|Default|GetDoor) (Math|Rotator|Lerp(Rotator) (Variables|Default|GetStartingRot) (Variables|Default|GetEndingRot) _doortrack) false false))))

(event EventBeginPlay
  (|CallParentFunction) ; This node is disabled and will not be called.\nDrag off pins to build functionality.
)

(event EventInteractDoor
  (CallFunction|SROpenDoor)
  (CallFunction|OCOpenDoor))

(fn ConstructionScript
  (|CallParentFunction))