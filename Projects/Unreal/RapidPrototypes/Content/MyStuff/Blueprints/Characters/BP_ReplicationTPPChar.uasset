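; Third-person character for testing replication, with debug keys for sprinting and opening doors through server events.
; Sprint sets max walk speed both locally and on the server to keep movement in sync.
; The door event line-traces forward from the capsule and sends an interact message to either door type.
; For the owner-only relevancy actor, it first makes the character the owner; the always-relevant door needs no ownership change.
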(event Custom|SR_Sprinting
  ;[0.15 0.15 0.15 0.5] CHANGES SERVER CODE - Sends request to server to allow the Server's Authoritative State copy of client 1's player to increase it's move speed.
  (Variables|/Script/Engine.CharacterMovementComponent|SetMaxWalkSpeed (Variables|Character|GetCharacterMovement) 1.2e+03))

(event Custom|SR_StopSprint
  ;[0.15 0.15 0.15 0.5] CHANGES SERVER CODE - Sends request to server to allow the Server's Authoritative State copy of client 1's player to increase it's move speed.
  (Variables|/Script/Engine.CharacterMovementComponent|SetMaxWalkSpeed (Variables|Character|GetCharacterMovement) 6e+02))

(event Custom|SR_OpenDoor
  (bind _hitactor (CallFunction|LineTracetoOpen))
  (bind _asbp_relevant_to_owner_only (Utilities|Casting|CastToBP_RelevantTo_OwnerOnly _hitactor)
    (:then
      (Actor|SetOwner _asbp_relevant_to_owner_only self)
      (Class|BPiDoorInterface|InteractDoor(Message) _asbp_relevant_to_owner_only))
    (:CastFailed
      (bind _asbp_door_always_relevant (Utilities|Casting|CastToBP_Door_AlwaysRelevant _hitactor))
      (Class|BPiDoorInterface|InteractDoor(Message) _asbp_door_always_relevant))))

(event Input|KeyboardEvents|DebugKeyE
  (params (Key :type Key%20Structure :default "None") (ActionValue :type Input%20Action%20Value%20Structure))
  (:Pressed
    (CallFunction|SROpenDoor)))

(event Input|KeyboardEvents|DebugKeyO
  (params (Key :type Key%20Structure :default "None") (ActionValue :type Input%20Action%20Value%20Structure))
  (bind _charactermovement (Variables|Character|GetCharacterMovement))
  ;[0.15 0.15 0.15 0.5] CHANGES THE LOCAL CLIENT CODE - This is local client's input changing it's properties and since the server expects this because of SR call below, the server and client remain in sync
  (:Pressed
    (CallFunction|SRSprinting)
    (Variables|/Script/Engine.CharacterMovementComponent|SetMaxWalkSpeed _charactermovement 1.2e+03))
  (:Released
    (CallFunction|SRStopSprint)
    (Variables|/Script/Engine.CharacterMovementComponent|SetMaxWalkSpeed _charactermovement 6e+02)))

(fn ConstructionScript
  (|CallParentFunction))

(fn LineTracetoOpen
  (bind _capsulecomponent (Variables|Default|GetCapsuleComponent))
  (bind _returnvalue (Transformation|GetWorldLocation _capsulecomponent))
  (bind (_outhit _returnvalue_2) (Collision|LineTraceByChannel _returnvalue (+ _returnvalue (* (Math|Vector|GetForwardVector _capsulecomponent) 7e+02)) "TraceTypeQuery1" false (Utilities|Array|MakeArray self) "ForDuration"))
  (if _returnvalue_2
    (return (.hitactor _outhit))
    (else
      (return 0))))