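; Player character Blueprint that exercises a component-based damage system, with a debug left-click attack and ragdoll death.
; The click sphere-traces ahead from the capsule, sends physical damage to the hit actor, and spawns an explosion if that call returns true.
; Health, healing and damage functions forward to BPCDamageComponent.
; Construction script binds the component's events: death enables mesh physics and disables input, while block, damage type and response print debug strings.
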(event Custom|Death%20Event
  (bind _mesh (Variables|Character|GetMesh))
  (Physics|SetSimulatePhysics _mesh true)
  (Collision|SetCollisionEnabled _mesh "QueryAndPhysics")
  (Input|DisableInput (Game|GetPlayerController 0)))

(event Custom|Blocked
  (params (canBeBlocked :type Boolean))
  (Development|PrintString "Blocked"))

(event Custom|DamageResponse
  (params (Response :type EDamageResponse%20Enum :default "None"))
  (Development|PrintString (Utilities|String|EnumtoString Response)))

(event Custom|DamageType
  (params (DamageType :type EDamageType%20Enum :default "None"))
  (Development|PrintString (Utilities|String|EnumtoString DamageType)))

(event Input|MouseEvents|DebugKeyLeftMouseButton
  (params (Key :type Key%20Structure :default "None") (ActionValue :type Input%20Action%20Value%20Structure))
  (bind _capsulecomponent (Variables|Default|GetCapsuleComponent))
  (bind _returnvalue (Transformation|GetWorldLocation _capsulecomponent))
  (:Pressed
    (bind (_outhit _returnvalue_2) (Class|KismetSystemLibrary|SphereTraceSinglebyProfile _returnvalue (+ (* (Math|Vector|GetForwardVector _capsulecomponent) 1.5e+02) _returnvalue) 25.0 "Pawn" false 0 "ForDuration" true "(R=1.000000,G=0.000000,B=0.000000,A=1.000000)" "(R=0.000000,G=1.000000,B=0.000000,A=1.000000)" 1.0))
    (if _returnvalue_2
      (bind _wasdamaged (Class|BPiDamagable|TakeDamage(Message) (.HitActor (Collision|BreakHitResult _outhit)) (Utilities|Struct|MakeDamageInfo 5e+01 "Physical" "HitReactionDefault" false false false false "None")))
      (if _wasdamaged
        (Effects|SpawnEmitteratLocation "/Game/StarterContent/Particles/P_Explosion.P_Explosion" (.Location (Collision|BreakHitResult _outhit)))))))

(fn ConstructionScript
  (bind _bpc_damagecomponent (Variables|Default|GetBPC_DamageComponent))
  (EventDispatchers|BindEventtoOnDeath (Variables|Default|GetBPC_DamageComponent) (EventDispatchers|CreateEvent :!event Custom|Death%20Event))
  (EventDispatchers|BindEventtoOnBlocked _bpc_damagecomponent (EventDispatchers|CreateEvent :!event Custom|Blocked))
  (EventDispatchers|BindEventtoOnDamageType _bpc_damagecomponent (EventDispatchers|CreateEvent :!event Custom|DamageType))
  (EventDispatchers|BindEventtoOnDamageResponse _bpc_damagecomponent (EventDispatchers|CreateEvent :!event Custom|DamageResponse)))

(fn GetCurrentHealth
  (return (Variables|/Game/MyStuff/Blueprints/DamageSystem/BPC_DamageComponent.BPC_DamageComponent_C|GetHealth (Variables|Default|GetBPC_DamageComponent))))

(fn GetMaxHealth
  (return (Variables|/Game/MyStuff/Blueprints/DamageSystem/BPC_DamageComponent.BPC_DamageComponent_C|GetMaxHealth (Variables|Default|GetBPC_DamageComponent))))

(fn Heal
  (params (HealingAmount :type Float%20%28double-precision%29))
  (bind _newhealth (Default|Heal (Variables|Default|GetBPC_DamageComponent) HealingAmount))
  (return _newhealth))

(fn TakeDamage
  (params (DamageInfo :type Damage%20Info%20Structure))
  (bind _wasdamaged (Default|TakeDamage (Variables|Default|GetBPC_DamageComponent) DamageInfo))
  (return _wasdamaged))