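; BP_Button_Parent_Toggle is a base interactive button that flips between enabled and disabled when the player interacts with its ButtonCollision component.
; ChangeButtonState stores the new state, calls the matching dispatcher and event, then passes the state to UpdateButtonVisuals.
; ButtonEnabled and ButtonDisabled are empty hooks, so behavior comes from child Blueprint overrides or dispatcher bindings.
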(event Custom|ButtonEnabled
  ;[0.15 0.15 0.15 0.5] Overwrite these in child blueprint or bind to event dispatcher depending on your requirements.
)

(event Custom|ButtonDisabled
  ;[0.15 0.15 0.15 0.5] Overwrite these in child blueprint or bind to event dispatcher depending on your requirements.
)

(event Custom|ChangeButtonState
  (params (NewState :type Boolean))
  ;[0.15 0.15 0.15 0.5] Update  button state and fire events/dispatchers
  (bind _output_get (Variables|Default|SetbButtonEnabled NewState))
  (if _output_get
    (Default|CallOnButtonEnabled)
    (CallFunction|ButtonEnabled)
    (else
      (Default|CallOnButtonDisabled)
      (CallFunction|ButtonDisabled)))
  (CallFunction|UpdateButtonVisuals (Variables|Default|GetbButtonEnabled)))

(event EventBeginPlay
  (|CallParentFunction) ; This node is disabled and will not be called.\nDrag off pins to build functionality.
)

(event Collision|EventActorBeginOverlap
  (params (OtherActor :type Actor%20Object%20Reference)))

(event EventTick
  (params (DeltaSeconds :type Float%20%28single-precision%29))
  (|CallParentFunction DeltaSeconds) ; This node is disabled and will not be called.\nDrag off pins to build functionality.
)

(event EventOnPlayerInteract
  (params (HitResult :type Hit%20Result%20Structure))
  ;[0.15 0.15 0.15 0.5] Toggle the button on and off when the player interacts
  (if (== (.HitComponent (Collision|BreakHitResult HitResult)) (Variables|Default|GetButtonCollision))
    (CallFunction|ChangeButtonState (not (Variables|Default|GetbButtonEnabled)))))

(fn ConstructionScript
  (|CallParentFunction))