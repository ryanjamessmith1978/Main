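; BP_BatteryPickup is a battery pickup Blueprint that adds a visual effect when collected.
; On WasCollected it attaches a pulse ring emitter to the player character's mesh at the spine_01 socket, waits briefly, then calls the parent's collection logic.
; Overlap and hit events are empty, with leftover debug print and upward impulse nodes left disconnected.
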(event OnComponentHit(PickupMesh)
  (params (HitComponent :type Primitive%20Component%20Object%20Reference) (OtherActor :type Actor%20Object%20Reference) (OtherComp :type Primitive%20Component%20Object%20Reference) (NormalImpulse :type Vector :default "0, 0, 0") (Hit :type Hit%20Result%20Structure%20%28by%20ref%29)))

(event EventWasCollected
  (Effects|SpawnEmitterAttached "/Game/Assets/Effects/P_Pulse_Ring.P_Pulse_Ring" (Variables|/Script/Engine.Character|GetMesh (Game|GetPlayerCharacter 0)) "spine_01" "0, 0, 0" "0, 0, 0" "1.000000,1.000000,1.000000" "SnapToTargetIncludingScale")
  (Utilities|FlowControl|Delay 0.3)
  (|CallParentFunction))

(event Collision|EventActorBeginOverlap
  (params (OtherActor :type Actor%20Object%20Reference)))

(fn ConstructionScript)