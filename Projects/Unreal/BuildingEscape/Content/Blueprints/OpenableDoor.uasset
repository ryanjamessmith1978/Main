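; Openable door actor that swings around its yaw axis when it receives open and close requests from its OpenDoor events.
; A RotateDoor timeline adds its yaw to the rotation saved at BeginPlay, and closing reverses it.
; A timeline event track plays a bird sound at the door once through a DoOnce.
; Closing also clears sound mix modifiers.
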(event OnOpenRequest(OpenDoor)
  (bind _rotate (Timeline|RotateDoor Play)
    (:Update
      (Transformation|SetActorRotation (Math|Rotator|CombineRotators (Math|Rotator|MakeRotator 0.0 0.0 _rotate) (Variables|Default|GetInitialDoorRotation))))
    (:SoundTiming
      (Utilities|FlowControl|DoOnce false
        (:Completed
          (Audio|PlaySoundatLocation "/Game/StarterContent/Audio/Starter_Birds01.Starter_Birds01" (Transformation|GetActorLocation)))))))

(event OnCloseRequest(OpenDoor)
  (Class|GameplayStatics|ClearSoundMixModifiers)
  (bind _rotate (Timeline|RotateDoor Reverse)
    (:Update
      (Transformation|SetActorRotation (Math|Rotator|CombineRotators (Math|Rotator|MakeRotator 0.0 0.0 _rotate) (Variables|Default|GetInitialDoorRotation))))
    (:SoundTiming
      (Utilities|FlowControl|DoOnce false
        (:Completed
          (Audio|PlaySoundatLocation "/Game/StarterContent/Audio/Starter_Birds01.Starter_Birds01" (Transformation|GetActorLocation)))))))

(event EventBeginPlay
  (Variables|Default|SetInitialDoorRotation (Transformation|GetActorRotation)))

(fn ConstructionScript)